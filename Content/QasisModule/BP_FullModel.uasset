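; BP_FullModel is an actor that detects small and large bags overlapping its trigger components and flags them through SmallBox and LargeBox.
; Overlaps on TW_L1 and TW_L2 cast to BP_Bag_1, and LW_L casts to BP_Bag_5, storing the bag and comparing it to a reference.
; A match sets the corresponding flag for a few seconds via a Delay, then clears it; both flags start false.
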(event `self.ReceiveBeginPlay`
  (set `self.smallBox` false)
  (set `self.largeBox` false))

(event `self.TW_L1.OnComponentBeginOverlap`
  (params (OverlappedComponent :type "PrimitiveComponent Object Reference") (OtherActor :type "Actor Object Reference") (OtherComp :type "PrimitiveComponent Object Reference") (OtherBodyIndex :type Integer) (bFromSweep :type Boolean) (SweepResult :type "HitResult Structure (by ref)"))
  (bind _asbp_bag_1 (cast `/Game/QasisModule/Meshes/BP_Bag_1` OtherActor))
  (bind _output_get (set `self.Small` _asbp_bag_1))
  (if (== _output_get "/Game/QasisModule/Meshes/BP_Bag_1.BP_Bag_1")
    (set `self.smallBox` true)
    (`KismetSystemLibrary.Delay` 3.0)
    (set `self.smallBox` false)))

(event `self.TW_L2.OnComponentBeginOverlap`
  (params (OverlappedComponent :type "PrimitiveComponent Object Reference") (OtherActor :type "Actor Object Reference") (OtherComp :type "PrimitiveComponent Object Reference") (OtherBodyIndex :type Integer) (bFromSweep :type Boolean) (SweepResult :type "HitResult Structure (by ref)"))
  (bind _asbp_bag_1 (cast `/Game/QasisModule/Meshes/BP_Bag_1` OtherActor))
  (bind _output_get (set `self.Small` _asbp_bag_1))
  (if (== _output_get "/Game/QasisModule/Meshes/BP_Bag_1.BP_Bag_1")
    (set `self.smallBox` true)
    (`KismetSystemLibrary.Delay` 3.0)
    (set `self.smallBox` false)))

(event `self.LW_L.OnComponentBeginOverlap`
  (params (OverlappedComponent :type "PrimitiveComponent Object Reference") (OtherActor :type "Actor Object Reference") (OtherComp :type "PrimitiveComponent Object Reference") (OtherBodyIndex :type Integer) (bFromSweep :type Boolean) (SweepResult :type "HitResult Structure (by ref)"))
  (bind _asbp_bag_5 (cast `/Game/QasisModule/Meshes/BP_Bag_5` OtherActor))
  (bind _output_get (set `self.Large` _asbp_bag_5))
  (if (== _output_get "/Game/QasisModule/Meshes/BP_Bag_5.BP_Bag_5")
    (set `self.largeBox` true)
    (`KismetSystemLibrary.Delay` 3.0)
    (set `self.largeBox` false)))

(fn `UserConstructionScript`)