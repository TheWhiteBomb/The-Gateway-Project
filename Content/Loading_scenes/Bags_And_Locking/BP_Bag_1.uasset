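; BP_Bag_1 is a grabbable bag in a VR loading scene that interacts with Locking actors it overlaps.
; On mesh overlap it passes its bag size enum to the Locking actor and shows that actor's plane, first hiding the previous one if the PC_Gateway controller's BagOverlapping flag is set.
; Ending overlap with the tracked actor hides its plane and clears the overlap state on bag, actor and controller.
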(event `self.ReceiveBeginPlay`
  (set `self.Overlap?` false)
  (set `self.false` false))

(event `self.staticMesh.OnComponentBeginOverlap`
  (params (OverlappedComponent :type "PrimitiveComponent Object Reference") (OtherActor :type "Actor Object Reference") (OtherComp :type "PrimitiveComponent Object Reference") (OtherBodyIndex :type Integer) (bFromSweep :type Boolean) (SweepResult :type "HitResult Structure (by ref)"))
  (bind _aspc_gateway (cast `/Game/Code/Core/PC_Gateway` (`GameplayStatics.GetPlayerController` 0) :!pure true))
  (if (`/Game/Code/Core/PC_Gateway.BagOverlapping` _aspc_gateway)
    (bind _aslocking (cast `/Game/Loading_scenes/Bags_And_Locking/Locking` (`self.colldier`)))
    (`SceneComponent.SetVisibility` (`/Game/Loading_scenes/Bags_And_Locking/Locking.Plane` _aslocking) false false))
  (bind _aslocking_2 (cast `/Game/Loading_scenes/Bags_And_Locking/Locking` OtherActor))
  (`/Game/Loading_scenes/Bags_And_Locking/Locking.DetectBagSize` _aslocking_2 (`self.enum`))
  (`SceneComponent.SetVisibility` (`/Game/Loading_scenes/Bags_And_Locking/Locking.Plane` _aslocking_2) true false)
  (set `/Game/Code/Core/PC_Gateway.BagOverlapping` true _aspc_gateway)
  (set `self.colldier` OtherActor))

(event `self.staticMesh.OnComponentEndOverlap`
  (params (OverlappedComponent :type "PrimitiveComponent Object Reference") (OtherActor :type "Actor Object Reference") (OtherComp :type "PrimitiveComponent Object Reference") (OtherBodyIndex :type Integer))
  (if (== OtherActor (`self.colldier`))
    (set `self.Overlap?` false)
    (bind _aslocking (cast `/Game/Loading_scenes/Bags_And_Locking/Locking` OtherActor))
    (set `/Game/Loading_scenes/Bags_And_Locking/Locking.AlreadyOverlapping` false _aslocking)
    (set `self.colldier` (`self.VarReset`))
    (`SceneComponent.SetVisibility` (`/Game/Loading_scenes/Bags_And_Locking/Locking.Plane` _aslocking) false false)
    (set `/Game/Code/Core/PC_Gateway.BagOverlapping` false (cast `/Game/Code/Core/PC_Gateway` (`GameplayStatics.GetPlayerController` 0) :!pure true))))

(event `self.GrabComponent.OnGrabbed`
  (if true
    _))

(fn `UserConstructionScript`)