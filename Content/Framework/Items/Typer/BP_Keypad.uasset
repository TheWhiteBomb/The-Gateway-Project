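; BP_Keypad is a keypad that builds a typed entry on a text display from button input.
; Buttonentered appends the value to EnterCodeText for plain key presses while CanEnter is true.
; Confirm, back and reset presses have no handling yet.
; A disconnected loop would give the fifteen child-actor BP_KeypadButtonActor buttons a reference to the keypad, but it never runs.
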(event `Button entered`
  (params (value :type Text) (`Confirmed?` :type Boolean) (Back :type Boolean) (Reset :type Boolean))
  (if `Confirmed?`
    _
    (elif Back
      _
      (elif Reset
        _
        (elif (`self.Can Enter`)
          (`TextRenderComponent.K2_SetText` (`self.EnterCodeText`) (`KismetTextLibrary.Conv_StringToText` (`KismetStringLibrary.Concat_StrStr` (`KismetTextLibrary.Conv_TextToString` (`TextRenderComponent.Text` (`self.EnterCodeText`))) (`KismetTextLibrary.Conv_TextToString` value)))))))))

(fn `UserConstructionScript`)