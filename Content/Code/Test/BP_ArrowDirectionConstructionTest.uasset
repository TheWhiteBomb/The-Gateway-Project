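; Test actor that compares ways of reversing an arrow component's direction, previewed in the construction script.
; For four source arrows, it adds an arrow using that source's world transform as relative transform, with altered rotation and color passed through LowerColor.
; Rotations use NegateRotator, FlipRotator, OppositeRotator and a zero-angle axis rotation around the negated forward vector.
; UsingInversedQuat takes the axis-angle route; its quaternion-inverse chain is unconnected.
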(fn `UserConstructionScript`
  (bind _usinginversedquat (`self.UsingInversedQuat`))
  (bind _usingcustom (`self.UsingCustom`))
  (bind _usinginvertrotator (`self.UsingInvertRotator`))
  (bind _usingownfliprotator (`self.UsingOwnFlipRotator`))
  (bind _returnvalue (`AddComponent|NODE_AddArrowComponent-0` :`RelativeTransform` (`KismetMathLibrary.MakeTransform` (.location (`SceneComponent.K2_GetComponentToWorld` _usinginversedquat)) (`KismetMathLibrary.RotatorFromAxisAndAngle` (`KismetMathLibrary.NegateVector` (`KismetMathLibrary.GetForwardVector` (.rotation (`SceneComponent.K2_GetComponentToWorld` _usinginversedquat))))) (.scale (`SceneComponent.K2_GetComponentToWorld` _usinginversedquat)))))
  (`ArrowComponent.SetArrowColor` _returnvalue (`self.LowerColor` (`KismetMathLibrary.Conv_ColorToLinearColor` (`ArrowComponent.ArrowColor` _usinginversedquat))))
  (bind _returnvalue_2 (`AddComponent|NODE_AddArrowComponent-1` :`RelativeTransform` (`KismetMathLibrary.MakeTransform` (.location (`SceneComponent.K2_GetComponentToWorld` _usinginvertrotator)) (`KismetMathLibrary.NegateRotator` (.rotation (`SceneComponent.K2_GetComponentToWorld` _usinginvertrotator))) (.scale (`SceneComponent.K2_GetComponentToWorld` _usinginvertrotator)))))
  (`ArrowComponent.SetArrowColor` _returnvalue_2 (`self.LowerColor` (`KismetMathLibrary.Conv_ColorToLinearColor` (`ArrowComponent.ArrowColor` _usinginvertrotator))))
  (bind _returnvalue_3 (`AddComponent|NODE_AddArrowComponent-2` :`RelativeTransform` (`KismetMathLibrary.MakeTransform` (.location (`SceneComponent.K2_GetComponentToWorld` _usingownfliprotator)) (`/Game/Code/ProjectLibraries/BPML_Global.Flip Rotator` (.rotation (`SceneComponent.K2_GetComponentToWorld` _usingownfliprotator))) (.scale (`SceneComponent.K2_GetComponentToWorld` _usingownfliprotator)))))
  (`ArrowComponent.SetArrowColor` _returnvalue_3 (`self.LowerColor` (`KismetMathLibrary.Conv_ColorToLinearColor` (`ArrowComponent.ArrowColor` _usingownfliprotator))))
  (bind _returnvalue_4 (`AddComponent|NODE_AddArrowComponent-3` :`RelativeTransform` (`KismetMathLibrary.MakeTransform` (.location (`SceneComponent.K2_GetComponentToWorld` _usingcustom)) (`/Game/Code/ProjectLibraries/BPML_Global.Opposite Rotator` (.rotation (`SceneComponent.K2_GetComponentToWorld` _usingcustom))) (.scale (`SceneComponent.K2_GetComponentToWorld` _usingcustom)))))
  (`ArrowComponent.SetArrowColor` _returnvalue_4 (`self.LowerColor` (`KismetMathLibrary.Conv_ColorToLinearColor` (`ArrowComponent.ArrowColor` _usingcustom)))))