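; BP_WallClock is a clutter actor that displays the current real-world time as text in GMT and MSK.
; Every Tick it reads the UTC time of day, derives MSK by adding a fixed three-hour timespan, and writes both labelled values to its TextRender component.
; An unconnected Append that would also show the date is left in the graph.
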(event `self.ReceiveTick`
  (params (DeltaSeconds :type "Float (single-precision)"))
  (bind _returnvalue (`KismetMathLibrary.GetTimeOfDay` (`KismetMathLibrary.UtcNow`)))
  (`TextRenderComponent.K2_SetText` (`self.TextRender`) (`KismetTextLibrary.Conv_StringToText` (`KismetStringLibrary.Concat_StrStr` "GMT: " (`KismetTextLibrary.Conv_TextToString` (`KismetTextLibrary.AsTimespan_Timespan` _returnvalue)) "\nMSK: " (`KismetTextLibrary.Conv_TextToString` (`KismetTextLibrary.AsTimespan_Timespan` (+ _returnvalue (`KismetMathLibrary.MakeTimespan` 0 3))))))))

(fn `UserConstructionScript`)