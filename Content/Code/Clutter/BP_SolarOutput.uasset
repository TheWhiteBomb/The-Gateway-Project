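; BP_SolarOutput is a clutter display that shows fake, fluctuating solar readouts on text components.
; Tick hashes game time, stepped every two seconds, with the shader-style fract(sin(x) * large constant) trick for stateless pseudo-random values.
; That value drives a one-decimal kW output on TextRender and a small angle-deviation figure in degrees on TextRender3.
; Both readings share the seed, so they change together, though the text is rebuilt every frame.
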(event `self.ReceiveTick`
  (params (DeltaSeconds :type "Float (single-precision)"))
  (bind _returnvalue (* (`KismetMathLibrary.Sin` (`KismetMathLibrary.Conv_IntToDouble` (`KismetMathLibrary.FFloor` (/ (`KismetSystemLibrary.GetGameTimeInSeconds`) 2.0)))) 43758.545312))
  (bind _returnvalue_2 (- _returnvalue (`KismetMathLibrary.FFloor` _returnvalue)))
  (`TextRenderComponent.K2_SetText` (`self.TextRender`) (`KismetTextLibrary.Conv_StringToText` (`KismetStringLibrary.Concat_StrStr` (`KismetStringLibrary.GetSubstring` (`KismetStringLibrary.Conv_DoubleToString` (/ (`KismetMathLibrary.Conv_IntToDouble` (`KismetMathLibrary.FFloor` (* (`KismetMathLibrary.Lerp` 57.0 63.0 _returnvalue_2) 10.0))) 10.0)) 0 4) "kW")))
  (`TextRenderComponent.K2_SetText` (`self.TextRender3`) (`KismetTextLibrary.Conv_StringToText` (`KismetStringLibrary.Concat_StrStr` "|n   -n     | ~= 0." (`KismetStringLibrary.Conv_IntToString` (`KismetMathLibrary.Abs_Int` (`KismetMathLibrary.Round` (`KismetMathLibrary.Lerp` 3.0 -2.0 _returnvalue_2)))) "°"))))

(fn `UserConstructionScript`)