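; Clutter prop of an air quality meter that animates its Cylinder component, likely the needle, with a purely procedural wobble.
; Each Tick, nested sines of game time, with a slowly oscillating frequency multiplier, produce an irregular value in a narrow low range.
; That value maps onto the Cylinder's relative yaw, so it flickers near one end of its half-turn dial range.
; No actual air quality data is read.
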(event `self.ReceiveBeginPlay`)

(event `self.ReceiveTick`
  (params (DeltaSeconds :type "Float (single-precision)"))
  (bind _returnvalue (`self.GetGameTimeSinceCreation`))
  (set `self.Value` (`KismetMathLibrary.Lerp` 0.05 0.02 (/ (+ (`KismetMathLibrary.Sin` (* (`KismetMathLibrary.Sin` (* _returnvalue (`KismetMathLibrary.Lerp` 0.41 0.17 (/ (+ (`KismetMathLibrary.Sin` (/ _returnvalue 8.73)) 1.0) 2.0)))) 2.25)) 1.0) 2.0)))
  (`SceneComponent.K2_SetRelativeRotation` (`self.Cylinder`) (`KismetMathLibrary.MakeRotator` 0.0 0.0 (`KismetMathLibrary.Lerp` -90.0 90.0 (`self.Value`))) false false))

(fn `UserConstructionScript`)