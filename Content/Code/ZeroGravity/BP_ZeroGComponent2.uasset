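; VR zero-gravity locomotion component that lets the player pull through space by grabbing handles, with unfinished wall-pushing.
; CloseHand sphere-overlaps at the controller, storing a BP_Handle grab or otherwise listing the hand as a wall hand; OpenHand releases it.
; Tick offsets the pawn so the gripping hand stays pinned to its grab point.
; Center-of-mass and shoulder estimates from HMD and floor are computed, but wall push and MovePlayer are stubs.
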(event `self.ReceiveTick`
  (params (DeltaSeconds :type "Float (single-precision)"))
  (bind _returnvalue (`GameplayStatics.GetPlayerPawn` 0))
  (`|ExecutionSequence`
    (:`then_0`)
    (:`then_1`
      (if (`KismetSystemLibrary.IsValid` (`self.HandleHand`))
        (`Actor.K2_SetActorLocation` _returnvalue (+ (`Actor.K2_GetActorLocation` _returnvalue) (- (`self.HandleLocation`) (`SceneComponent.K2_GetComponentLocation` (`self.HandleHand`)))) false false)
        (elif (`KismetArrayLibrary.Array_IsNotEmpty` (`self.WallHands`))
          _)))))

(fn `BeginPlay`
  (params (LMotionController :type "MotionControllerComponent Object Reference") (RMotionController :type "MotionControllerComponent Object Reference"))
  (set `self.LeftMotionController` LMotionController)
  (set `self.RightMotionController` RMotionController))

(fn `Close Hand`
  (params (`Closed Hand` :type "MotionControllerComponent Object Reference"))
  (bind _outactors (`KismetSystemLibrary.SphereOverlapActors` (`SceneComponent.K2_GetComponentLocation` `Closed Hand`) 10.0 (`|MakeArray` "ObjectTypeQuery2" :!type "EObjectTypeQuery Enum")))
  (for (_array_element _array_index) _outactors
    (if (== (`GameplayStatics.GetObjectClass` _array_element) "/Game/Code/ZeroGravity/BP_Handle.BP_Handle_C")
      (bind _output_get (set `self.HandleHand` `Closed Hand`))
      (set `self.HandleLocation` (`SceneComponent.K2_GetComponentLocation` _output_get))
      (break)
      (elif (== _array_index (`KismetArrayLibrary.Array_LastIndex` _outactors))
        (`KismetArrayLibrary.Array_Add` (`self.WallHands`) `Closed Hand`)
        (break)))))

(fn `GetMovementDirection`
  (bind _hmddata (`HeadMountedDisplayFunctionLibrary.GetHMDData` (`/Game/Code/ProjectLibraries/BPML_Global.GetStreamingLevel`)))
  (set `self.HMD Location` (`.Position` (break `XRHMDData` _hmddata)))
  (bind _outtransform (`HeadMountedDisplayFunctionLibrary.GetTrackingOriginTransform` (`HeadMountedDisplayFunctionLibrary.GetTrackingOrigin`)))
  (set `self.FloorLocation` (.location _outtransform))
  (set `self.Initial CenterOfMass` (+ (`self.HMD Location`) (* (`KismetMathLibrary.GetDirectionUnitVector` (`self.HMD Location`) (`self.FloorLocation`)) 84.0)))
  (set `self.ShoulderHeight` (+ (`self.HMD Location`) (* (`KismetMathLibrary.GetDirectionUnitVector` (`self.HMD Location`) (`self.FloorLocation`)) 33.0))))

(fn `MovePlayer`)

(fn `OpenHand`
  (params (OpenedHand :type "MotionControllerComponent Object Reference"))
  (if (== OpenedHand (`self.HandleHand`))
    (set `self.HandleHand` null)
    (else
      (`KismetArrayLibrary.Array_RemoveItem` (`self.WallHands`) OpenedHand))))

(fn `PushWall`
  (params (PushingHand :type "MotionControllerComponent Object Reference"))
  (bind _returnvalue (`Actor.GetActorRightVector` (`GameplayStatics.GetPlayerPawn` 0)))
  (set `self.RShoulder` (+ (`self.ShoulderHeight`) (* _returnvalue 20.0)))
  (set `self.LShoulder` (+ (`self.ShoulderHeight`) (* (* _returnvalue -1.0) 20.0))))