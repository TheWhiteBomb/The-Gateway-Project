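; VR zero-gravity locomotion component that moves the player pawn by handle grabs and wall pushes.
; A closing hand grabs an overlapped BP_Handle to drag the pawn, which drifts at hand velocity after release.
; Otherwise the hand is tracked for pushing, and HandOverlap splits its velocity into Linear and Torque, which Tick applies to location and control rotation.
; Push math is unfinished, with zero-vector placeholders, unreached center-of-mass code and debug prints.
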(event `self.ReceiveBeginPlay`)

(event `self.ReceiveTick`
  (params (DeltaSeconds :type "Float (single-precision)"))
  (bind _returnvalue (`GameplayStatics.GetPlayerController` 0))
  (bind _returnvalue_2 (`GameplayStatics.GetPlayerPawn` 0))
  (bind _returnvalue_3 (`GameplayStatics.GetPlayerPawn` 0))
  (bind _returnvalue_4 (`GameplayStatics.GetPlayerPawn` 0))
  (bind _torque (`self.Torque`))
  (bind _returnvalue_5 (`Actor.K2_GetActorLocation` _returnvalue_4))
  (bind _returnvalue_6 (+ (.roll (`Controller.GetControlRotation` _returnvalue)) (.x _torque)))
  (bind _returnvalue_7 (+ (.pitch (`Controller.GetControlRotation` _returnvalue)) (.y _torque)))
  (bind _returnvalue_8 (+ (.yaw (`Controller.GetControlRotation` _returnvalue)) (.z _torque)))
  (if (`KismetArrayLibrary.Array_IsValidIndex` (`self.PushingHands`))
    (for (_array_element _array_index) (`self.PushingHands`)
      (`KismetArrayLibrary.Array_Set` (`self.PushLocations`) _array_index (make `/Game/Code/ZeroGravity/S_PushLocationsAndHands` _array_element (`SceneComponent.K2_GetComponentLocation` _array_element) (`.PushLocation1_7_3225B2B341D7132124D9129078D7F34D` (break `/Game/Code/ZeroGravity/S_PushLocationsAndHands` (`|GetArrayItem` (`self.PushLocations`) _array_index)))))))
  (`/Engine/EditorBlueprintResources/StandardMacros.IsValid` (`self.GrabbedHandle`)
    (:`Is Valid`
      (`Actor.K2_SetActorLocation` _returnvalue_3 (+ (`Actor.K2_GetActorLocation` _returnvalue_3) (- (`self.GrabLocation`) (`SceneComponent.K2_GetComponentLocation` (`self.HoldingHand`)))) false false))
    (:`Is Not Valid`
      (if (`self.HandleVelocity`)
        (`Actor.K2_SetActorLocation` _returnvalue_4 (`KismetMathLibrary.VLerp` _returnvalue_5 (+ _returnvalue_5 (`self.MovementDirection`)) DeltaSeconds) false false)
        (elif (`self.PushedOffWall`)
          (`Controller.SetControlRotation` _returnvalue (`KismetMathLibrary.MakeRotator` _returnvalue_6 _returnvalue_7 _returnvalue_8))
          ; it it doesn't work change cross product to unit direction
          (`Actor.K2_SetActorLocation` _returnvalue_2 (+ (`Actor.K2_GetActorLocation` _returnvalue_2) (`self.Linear`)) false false)
          (`KismetSystemLibrary.PrintString` (`KismetStringLibrary.Conv_RotatorToString` (`KismetMathLibrary.MakeRotator` _returnvalue_6 _returnvalue_7 _returnvalue_8)))
          (`KismetSystemLibrary.PrintString` (`KismetStringLibrary.Conv_VectorToString` _torque) true true (struct :`R` 1.0 :`G` 0.11444 :`A` 1.0)))))))

(fn `GrabAwayFromGrabComponent`
  (params (NewHand :type "MotionControllerComponent Object Reference"))
  (bind _pushinghands (`self.PushingHands`))
  (bind (_outactors _returnvalue) (`KismetSystemLibrary.SphereOverlapActors` (`SceneComponent.K2_GetComponentLocation` NewHand) 10.0 (`|MakeArray` "ObjectTypeQuery2" :!type "EObjectTypeQuery Enum") "/Game/Code/ZeroGravity/BP_Handle.BP_Handle_C"))
  (if _returnvalue
    (set `self.GrabbedHandle` (`|GetArrayItem` _outactors))
    (set `self.HoldingHand` NewHand)
    (set `self.GrabLocation` (`SceneComponent.K2_GetComponentLocation` NewHand))
    (set `self.PushedOffWall` false)
    (set `self.HandleVelocity` false)
    (else
      (for (_array_element _array_index) _pushinghands
        (if (== _array_element NewHand)
          (break)
          (elif (== (`KismetArrayLibrary.Array_LastIndex` _pushinghands) _array_index)
            (`KismetArrayLibrary.Array_Add` (`self.PushingHands`) NewHand :!label _label))))
      (if (`KismetArrayLibrary.Array_IsEmpty` _pushinghands)
        (goto _label)))))

(fn `HandOverlap`
  (params (`Overlapped hand` :type "MotionControllerComponent Object Reference"))
  (locals (PushTick :type "Vector Structure" :default (0.0 0.0 0.0)))
  (bind _returnvalue (`GameplayStatics.GetPlayerPawn` 0))
  (bind _movementdirection (`self.MovementDirection`))
  (bind _returnvalue_2 (`Actor.GetActorRightVector` _returnvalue))
  (bind _returnvalue_3 (`Actor.K2_GetActorLocation` (`GameplayStatics.GetPlayerPawn` 0)))
  (bind _returnvalue_4 (* _movementdirection (`KismetMathLibrary.Vector_CosineAngle2D` _movementdirection)))
  (for _array_element (`self.PushingHands`)
    (if (== _array_element `Overlapped hand`)
      (for _array_element_2 (`self.PushLocations`)
        (bind (_pushhand _pushlocation1 _pushlocation2) (break `/Game/Code/ZeroGravity/S_PushLocationsAndHands` _array_element_2))
        (if (== _array_element _pushhand)
          (set `self.MovementDirection` (+ (/ (- _pushlocation2 _pushlocation1) (`GameplayStatics.GetWorldDeltaSeconds`)) (`self.MovementDirection`)))
          (break)))
      (for _array_element_3 (`Actor.K2_GetComponentsByClass` (`self.GetOwner`) "/Script/HeadMountedDisplay.MotionControllerComponent")
        (if (`KismetStringLibrary.EqualEqual_StrStr` (`KismetSystemLibrary.GetObjectName` _array_element_3) "MotionControllerLeftGrip")
          (bind _hmddata (`HeadMountedDisplayFunctionLibrary.GetHMDData` (`/Game/Code/ProjectLibraries/BPML_Global.GetStreamingLevel`)))
          (set `self.TrackingOrigin` (`KismetMathLibrary.MakeTransform` (`.Position` (break `XRHMDData` _hmddata)) (`Actor.K2_GetActorRotation` (`GameplayStatics.GetPlayerPawn` 0))))
          (set `self.PushedOffWall` true)
          (set `self.HandleVelocity` false)
          (bind _outtransform (`HeadMountedDisplayFunctionLibrary.GetTrackingOriginTransform` "Stage"))
          (bind _returnvalue_5 (`KismetMathLibrary.GetDirectionUnitVector` (.location (`self.TrackingOrigin`)) (.location _outtransform)))
          (bind _returnvalue_6 (* (`self.MovementDirection`) (`KismetMathLibrary.Vector_CosineAngle2D` (`self.MovementDirection`) (`KismetMathLibrary.GetDirectionUnitVector` (+ _returnvalue_3 (* _returnvalue_5 12.0)) (+ (+ _returnvalue_3 (* _returnvalue_5 10.0)) (* (`KismetMathLibrary.Normal` (`KismetMathLibrary.GetDirectionUnitVector` _returnvalue_2 (`KismetMathLibrary.Quat_RotateVector` (`KismetMathLibrary.Conv_RotatorToQuaternion` (`Actor.K2_GetActorRotation` _returnvalue)) _returnvalue_2))) 20.0))))))
          ; it it doesn't work change cross product to unit direction
          (set `self.Torque` (* _returnvalue_6 (`GameplayStatics.GetWorldDeltaSeconds`)))
          (set `self.Linear` (* (- (`self.MovementDirection`) _returnvalue_6) (`GameplayStatics.GetWorldDeltaSeconds`)))
          (else
            (bind _hmddata_2 (`HeadMountedDisplayFunctionLibrary.GetHMDData` (`/Game/Code/ProjectLibraries/BPML_Global.GetStreamingLevel`)))
            (set `self.TrackingOrigin` (`KismetMathLibrary.MakeTransform` (`.Position` (break `XRHMDData` _hmddata_2)) (`Actor.K2_GetActorRotation` (`GameplayStatics.GetPlayerPawn` 0))))
            (set `self.PushedOffWall` true)
            (set `self.HandleVelocity` false)
            (bind _outtransform_2 (`HeadMountedDisplayFunctionLibrary.GetTrackingOriginTransform` "Stage"))
            ; it it doesn't work change cross product to unit direction
            (set `self.Torque` (* _returnvalue_4 (`GameplayStatics.GetWorldDeltaSeconds`)))
            (set `self.Linear` (* (- (`self.MovementDirection`) _returnvalue_4) (`GameplayStatics.GetWorldDeltaSeconds`))))))
      (break))))

(fn `OpenAwayFromGrabComponent`
  (params (OpenHand :type "MotionControllerComponent Object Reference"))
  (if (== OpenHand (`self.HoldingHand`))
    (set `self.GrabbedHandle` null)
    (set `self.MovementDirection` (/ (- (`self.GrabLocation`) (`SceneComponent.K2_GetComponentLocation` (`self.HoldingHand`))) (`GameplayStatics.GetWorldDeltaSeconds`)))
    (set `self.HoldingHand` null)
    (set `self.HandleVelocity` true)
    (else
      (for _array_element (`self.PushingHands`)
        (if (== OpenHand _array_element)
          (`KismetArrayLibrary.Array_RemoveItem` (`self.PushingHands`) _array_element)
          (break))))))

(fn `SetCameraReferance`
  (params (CameraRef :type "CameraActor Object Reference")))