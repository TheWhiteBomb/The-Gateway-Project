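; BP_ModuleBase is a base module actor that registers itself as the Module on the Gateway game instance at BeginPlay.
; BoxOverlap and EndOverlap functions maintain a duplicate-free OverlappingBoxes list of BP_GWBoxBase actors.
; EndOverlap removes a box only once it is absent from the overlapping-actors query.
; Begin and end overlap events for five box components are empty here, so neither function is called in this graph.
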(event `self.ReceiveBeginPlay`
  (bind (_asgateway_game_instance _bsuccess) (`/Game/Code/ProjectLibraries/BPML_Global.GetGatewayGameInstance`))
  (if _bsuccess
    (set `/Game/Code/Persistent/GatewayGameInstance.Module` self _asgateway_game_instance)))

(event `self.Box1.OnComponentEndOverlap`
  (params (OverlappedComponent :type "PrimitiveComponent Object Reference") (OtherActor :type "Actor Object Reference") (OtherComp :type "PrimitiveComponent Object Reference") (OtherBodyIndex :type Integer)))

(event `self.Box2.OnComponentEndOverlap`
  (params (OverlappedComponent :type "PrimitiveComponent Object Reference") (OtherActor :type "Actor Object Reference") (OtherComp :type "PrimitiveComponent Object Reference") (OtherBodyIndex :type Integer)))

(event `self.Box3.OnComponentEndOverlap`
  (params (OverlappedComponent :type "PrimitiveComponent Object Reference") (OtherActor :type "Actor Object Reference") (OtherComp :type "PrimitiveComponent Object Reference") (OtherBodyIndex :type Integer)))

(event `self.Box4.OnComponentEndOverlap`
  (params (OverlappedComponent :type "PrimitiveComponent Object Reference") (OtherActor :type "Actor Object Reference") (OtherComp :type "PrimitiveComponent Object Reference") (OtherBodyIndex :type Integer)))

(event `self.Box.OnComponentEndOverlap`
  (params (OverlappedComponent :type "PrimitiveComponent Object Reference") (OtherActor :type "Actor Object Reference") (OtherComp :type "PrimitiveComponent Object Reference") (OtherBodyIndex :type Integer)))

(event `self.Box1.OnComponentBeginOverlap`
  (params (OverlappedComponent :type "PrimitiveComponent Object Reference") (OtherActor :type "Actor Object Reference") (OtherComp :type "PrimitiveComponent Object Reference") (OtherBodyIndex :type Integer) (bFromSweep :type Boolean) (SweepResult :type "HitResult Structure (by ref)")))

(event `self.Box2.OnComponentBeginOverlap`
  (params (OverlappedComponent :type "PrimitiveComponent Object Reference") (OtherActor :type "Actor Object Reference") (OtherComp :type "PrimitiveComponent Object Reference") (OtherBodyIndex :type Integer) (bFromSweep :type Boolean) (SweepResult :type "HitResult Structure (by ref)")))

(event `self.Box3.OnComponentBeginOverlap`
  (params (OverlappedComponent :type "PrimitiveComponent Object Reference") (OtherActor :type "Actor Object Reference") (OtherComp :type "PrimitiveComponent Object Reference") (OtherBodyIndex :type Integer) (bFromSweep :type Boolean) (SweepResult :type "HitResult Structure (by ref)")))

(event `self.Box4.OnComponentBeginOverlap`
  (params (OverlappedComponent :type "PrimitiveComponent Object Reference") (OtherActor :type "Actor Object Reference") (OtherComp :type "PrimitiveComponent Object Reference") (OtherBodyIndex :type Integer) (bFromSweep :type Boolean) (SweepResult :type "HitResult Structure (by ref)")))

(event `self.Box.OnComponentBeginOverlap`
  (params (OverlappedComponent :type "PrimitiveComponent Object Reference") (OtherActor :type "Actor Object Reference") (OtherComp :type "PrimitiveComponent Object Reference") (OtherBodyIndex :type Integer) (bFromSweep :type Boolean) (SweepResult :type "HitResult Structure (by ref)")))

(fn `BoxOverlap`
  (params (`Other Actor` :type "Actor Object Reference") (OverlappingComp :type "PrimitiveComponent Object Reference"))
  (if (`.bSuccess` (cast `/Game/Code/Boxes/Base/BP_GWBoxBase` `Other Actor` :!pure true))
    (if (not (`KismetArrayLibrary.Array_Contains` (`self.OverlappingBoxes`) `Other Actor`))
      (`KismetArrayLibrary.Array_Add` (`self.OverlappingBoxes`) `Other Actor`))))

(fn `EndOverlap`
  (params (OtherActor :type "Actor Object Reference") (`Overlapping comp` :type "PrimitiveComponent Object Reference"))
  (if (`.bSuccess` (cast `/Game/Code/Boxes/Base/BP_GWBoxBase` OtherActor :!pure true))
    (if (not (`KismetArrayLibrary.Array_Contains` (`self.GetOverlappingActors` "/Script/Engine.Actor") OtherActor))
      (`KismetArrayLibrary.Array_RemoveItem` (`self.OverlappingBoxes`) OtherActor))))

(fn `UserConstructionScript`)