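; BP_BindActors is a grabbable box that snaps and attaches to other BP_BindActors when dropped.
; Binder/Binded overlaps with HitBox-tagged components queue pairs in OverlappedComponents; construction also spawns tagged spheres from VelcroSocketConfig.
; On drop, the first eligible pair drives dot/cross quaternion axis alignment, offsets the mesh and attaches it to the other cube.
; Each eligible pair moves to ConnectedComponents on both actors, preventing repeat binding; no unbind logic runs.
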(event `self.GrabComponent.OnDropped`
  (bind _returnvalue (`SceneComponent.GetForwardVector` (`self.CubeMesh`)))
  (bind _returnvalue_2 (`SceneComponent.GetUpVector` (`self.CubeMesh`)))
  (bind (_keypin _valuepin) (`|MapForEach` (`self.OverlappedComponents`))
    (:`then`
      (bind (_asbp_bind_actors _bsuccess) (cast `/Game/Code/Boxes/BP_BindActors` (`ActorComponent.GetOwner` _valuepin) :!pure true))
      (if (and (`BlueprintMapLibrary.Map_Contains` (`self.ConnectedComponents`) _keypin) _bsuccess)
        _
        (elif (not (`BlueprintMapLibrary.Map_Contains` (`/Game/Code/Boxes/BP_BindActors.ConnectedComponents` _asbp_bind_actors) _valuepin))
          (`|ExecutionSequence`
            (:`then_0`
              (`/Engine/EditorBlueprintResources/StandardMacros.DoOnce` false :!label _label
                (:`Completed`
                  (`|ExecutionSequence`
                    (:`then_0`
                      (set `self.ConnectedParent` _asbp_bind_actors)
                      (bind _cubemesh (`/Game/Code/Boxes/BP_BindActors.CubeMesh` _asbp_bind_actors))
                      (bind _returnvalue_3 (`SceneComponent.GetForwardVector` _cubemesh))
                      (bind _returnvalue_4 (`KismetMathLibrary.Dot_VectorVector` _returnvalue _returnvalue_3))
                      (bind _returnvalue_5 (`KismetMathLibrary.InRange_FloatFloat` _returnvalue_4 -0.5 0.5))
                      (if _returnvalue_5
                        (bind _returnvalue_6 (`SceneComponent.GetUpVector` _cubemesh))
                        (bind _returnvalue_7 (`KismetMathLibrary.Dot_VectorVector` _returnvalue_2 _returnvalue_6))
                        (bind _returnvalue_8 (select `bool` (`KismetMathLibrary.InRange_FloatFloat` _returnvalue_7 -0.5 0.5) :`false` _returnvalue_2))
                        (bind _returnvalue_9 (select `bool` (> _returnvalue_7 0.0) :`false` (* _returnvalue_8 -1.0) :`true` _returnvalue_8))
                        (bind _returnvalue_10 (/ (`KismetMathLibrary.DegAcos` (`KismetMathLibrary.Dot_VectorVector` _returnvalue_9 _returnvalue_6)) 2.0))
                        (bind _returnvalue_11 (`KismetMathLibrary.Quat_Rotator` (`KismetMathLibrary.MakeQuat` (.x (* (`KismetMathLibrary.Cross_VectorVector` _returnvalue_9 _returnvalue_6) (`KismetMathLibrary.DegSin` _returnvalue_10))) (.y (* (`KismetMathLibrary.Cross_VectorVector` _returnvalue_9 _returnvalue_6) (`KismetMathLibrary.DegSin` _returnvalue_10))) (.z (* (`KismetMathLibrary.Cross_VectorVector` _returnvalue_9 _returnvalue_6) (`KismetMathLibrary.DegSin` _returnvalue_10))) (`KismetMathLibrary.DegCos` _returnvalue_10))))
                        (`SceneComponent.K2_AddWorldRotation` (`self.CubeMesh`) _returnvalue_11 false false)
                        (bind _returnvalue_12 (select `bool` _returnvalue_5 :`false` _returnvalue))
                        (bind _returnvalue_13 (select `bool` (> _returnvalue_4 0.0) :`false` (* _returnvalue_12 -1.0) :`true` _returnvalue_12))
                        (bind _returnvalue_14 (/ (`KismetMathLibrary.DegAcos` (`KismetMathLibrary.Dot_VectorVector` _returnvalue_13 _returnvalue_3)) 2.0))
                        (bind _returnvalue_15 (`KismetMathLibrary.Quat_Rotator` (`KismetMathLibrary.MakeQuat` (.x (* (`KismetMathLibrary.Cross_VectorVector` _returnvalue_13 _returnvalue_3) (`KismetMathLibrary.DegSin` _returnvalue_14))) (.y (* (`KismetMathLibrary.Cross_VectorVector` _returnvalue_13 _returnvalue_3) (`KismetMathLibrary.DegSin` _returnvalue_14))) (.z (* (`KismetMathLibrary.Cross_VectorVector` _returnvalue_13 _returnvalue_3) (`KismetMathLibrary.DegSin` _returnvalue_14))) (`KismetMathLibrary.DegCos` _returnvalue_14))))
                        (`SceneComponent.K2_SetWorldRotation` (`self.CubeMesh`) _returnvalue_15 false false)
                        (else
                          (`SceneComponent.K2_AddWorldRotation` (`self.CubeMesh`) _returnvalue_15 false false)
                          (`SceneComponent.K2_SetWorldRotation` (`self.CubeMesh`) _returnvalue_11 false false))))
                    (:`then_1`
                      (`SceneComponent.K2_SetWorldLocation` (`self.CubeMesh`) (+ (`SceneComponent.K2_GetComponentLocation` (`self.CubeMesh`)) (- (`SceneComponent.K2_GetComponentLocation` _valuepin) (`SceneComponent.K2_GetComponentLocation` _keypin))) false false)
                      (`SceneComponent.K2_AttachToComponent` (`self.CubeMesh`) (`/Game/Code/Boxes/BP_BindActors.CubeMesh` _asbp_bind_actors) "None" "KeepWorld" "KeepWorld" "KeepWorld" true))))))
            (:`then_1`
              (`BlueprintMapLibrary.Map_Add` (`self.ConnectedComponents`) _keypin _valuepin)
              (`BlueprintMapLibrary.Map_Remove` (`self.OverlappedComponents`) _keypin)
              (`BlueprintMapLibrary.Map_Remove` (`/Game/Code/Boxes/BP_BindActors.OverlappedComponents` _asbp_bind_actors) _valuepin)
              (`BlueprintMapLibrary.Map_Add` (`/Game/Code/Boxes/BP_BindActors.ConnectedComponents` _asbp_bind_actors) _valuepin _keypin))))))
    (:`CompletedPin`
      (goto _label :!via `Reset`))))

(event `self.GrabComponent.OnGrabbed`)

(event `self.ReceiveBeginPlay`)

(event `self.ReceiveTick`
  (params (DeltaSeconds :type "Float (single-precision)"))
  (`SceneComponent.K2_SetWorldLocation` (`self.CubeMesh`) (`SceneComponent.K2_GetComponentLocation` (`self.CubeMesh`)) true false))

(event `HelloThisIsMyTestEVent`
  (params (OverlappedComponent :type "PrimitiveComponent Object Reference") (OtherActor :type "Actor Object Reference") (OtherComp :type "PrimitiveComponent Object Reference") (OtherBodyIndex :type Integer) (bFromSweep :type Boolean) (SweepResult :type "HitResult Structure (by ref)")))

(event `self.Binder1.OnComponentBeginOverlap`
  (params (OverlappedComponent :type "PrimitiveComponent Object Reference") (OtherActor :type "Actor Object Reference") (OtherComp :type "PrimitiveComponent Object Reference") (OtherBodyIndex :type Integer) (bFromSweep :type Boolean) (SweepResult :type "HitResult Structure (by ref)"))
  (`self.BoxOverlapWhileHolding` OverlappedComponent OtherComp))

(event `self.Binded1.OnComponentBeginOverlap`
  (params (OverlappedComponent :type "PrimitiveComponent Object Reference") (OtherActor :type "Actor Object Reference") (OtherComp :type "PrimitiveComponent Object Reference") (OtherBodyIndex :type Integer) (bFromSweep :type Boolean) (SweepResult :type "HitResult Structure (by ref)"))
  (`self.BoxOverlapWhileHolding` OverlappedComponent OtherComp))

(event `self.Binder2.OnComponentBeginOverlap`
  (params (OverlappedComponent :type "PrimitiveComponent Object Reference") (OtherActor :type "Actor Object Reference") (OtherComp :type "PrimitiveComponent Object Reference") (OtherBodyIndex :type Integer) (bFromSweep :type Boolean) (SweepResult :type "HitResult Structure (by ref)"))
  (`self.BoxOverlapWhileHolding` OverlappedComponent OtherComp))

(event `self.Binded2.OnComponentBeginOverlap`
  (params (OverlappedComponent :type "PrimitiveComponent Object Reference") (OtherActor :type "Actor Object Reference") (OtherComp :type "PrimitiveComponent Object Reference") (OtherBodyIndex :type Integer) (bFromSweep :type Boolean) (SweepResult :type "HitResult Structure (by ref)"))
  (`self.BoxOverlapWhileHolding` OverlappedComponent OtherComp))

(fn `BoxOverlapWhileHolding`
  (params (`Overlapped Comp` :type "PrimitiveComponent Object Reference") (`Other Comp` :type "PrimitiveComponent Object Reference"))
  (bind (_asbp_bind_actors _bsuccess) (cast `/Game/Code/Boxes/BP_BindActors` (`ActorComponent.GetOwner` `Other Comp`) :!pure true))
  (if (and (`KismetArrayLibrary.Array_Contains` (`ActorComponent.ComponentTags` `Other Comp`) "HitBox") _bsuccess (!= `Other Comp` self))
    (if (not (`BlueprintMapLibrary.Map_Contains` (`/Game/Code/Boxes/BP_BindActors.ConnectedComponents` _asbp_bind_actors) `Other Comp`))
      (`BlueprintMapLibrary.Map_Add` (`self.OverlappedComponents`) `Overlapped Comp` `Other Comp`))))

(fn `UserConstructionScript`
  (bind _velcrosocketconfig (`self.VelcroSocketConfig`))
  (bind _keys (`BlueprintMapLibrary.Map_Keys` _velcrosocketconfig))
  (for _array_element _keys
    (bind (_tag _isconnected _fallbackposition) (break `/Game/Core/Structures/S_ConnectionPoint` (`BlueprintMapLibrary.Map_Find` _velcrosocketconfig _array_element)))
    (bind _returnvalue (`AddComponent|NODE_AddSphereComponent-1` :`RelativeTransform` _fallbackposition))
    (`SceneComponent.K2_AttachToComponent` _returnvalue (`self.CubeMesh`) _array_element "KeepRelative" "KeepRelative" "KeepRelative" true)
    (`/Game/Code/ProjectLibraries/BPML_Global.AddTag` _returnvalue _tag)
    (add `PrimitiveComponent.OnComponentBeginOverlap` _returnvalue (`|CreateDelegate` :!event `HelloThisIsMyTestEVent`))))