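; BP_TaskFinalizer is a Blueprint that credits task progress when a box of a given type is checked.
; CheckBox ignores one excluded enum type, then loops over the task entries held in the wrist gadget's TextHandler.
; Each task's BoxType and BoxTypeExtension are compared independently with that type, and each match adds one progress to its segment through TaskAddProgress.
; The event graph and construction script are empty.
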(fn `CheckBox`
  (params (Type :type "/Game/Core/Enums/E_BagType Enum" :default "NewEnumerator0"))
  (locals (CurrentTask :type "/Game/Core/Structures/S_Print Structure"))
  (if (`|EnumInequality` Type "NewEnumerator14")
    (for _array_element (`/Game/Code/wristGadget/RenderTargets/BP_text.Text` (`/Game/Code/wristGadget/BP_wristGadget.Text Handler` (`/Game/Code/ProjectLibraries/BPML_Global.GetWristGadget`)))
      (bind _output_get (set `local.CurrentTask` _array_element))
      (`|ExecutionSequence`
        (:`then_0`
          (bind (_taskname _taskprogress _taskrequired _taskprogressextension _taskrequiredextension _hasextension _boxtype _boxtypeextension) (break `/Game/Core/Structures/S_Print` _output_get))
          (if (`|EnumEquality` _boxtype (`local.Type`))
            (set `local.CurrentTask` (`/Game/Code/ProjectLibraries/BPML_Global.TaskAddProgress` (`local.CurrentTask`)))))
        (:`then_1`
          (if (`|EnumEquality` _boxtypeextension (`local.Type`))
            (set `local.CurrentTask` (`/Game/Code/ProjectLibraries/BPML_Global.TaskAddProgress` (`local.CurrentTask`) 1 "NewEnumerator1"))))))))

(fn `UserConstructionScript`)