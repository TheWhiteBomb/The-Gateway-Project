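; Physics box with a contents label that snaps and locks to other constraint boxes when dropped, with toggleable zero gravity.
; Construction builds locked physics constraints with sphere and arrow markers on configured face points.
; On drop, sphere traces find the nearest free constraint on another box, and a box trace vets the target pose.
; It then aligns and constrains that box, recording links on both sides plus soft attachments for other overlapped free points.
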(event `self.ReceiveBeginPlay`
  (set `self.Constraints` (`self.K2_GetComponentsByClass` "/Script/Engine.PhysicsConstraintComponent")))

(event `self.ReceiveTick`
  (params (DeltaSeconds :type "Float (single-precision)"))
  (bind _returnvalue (not (`self.ZeroGravity`)))
  (`PrimitiveComponent.SetEnableGravity` (`self.Center`) _returnvalue)
  (`PrimitiveComponent.SetEnableGravity` (`self.CollisionEnforcer`) _returnvalue))

(event `self.GrabComponent.OnDropped`
  (`self.UpdateCollisionAttachments`))

(fn `AddSoftAttachment`
  (params (SelfConstraint :type "PhysicsConstraintComponent Object Reference") (Other :type "/Game/Code/Boxes/BP_ConstraintBox Object Reference") (OtherConstraint :type "PhysicsConstraintComponent Object Reference"))
  (`self.AttachOtherFromSelf` (make `/Game/Core/Structures/S_ConstraintData` "NewEnumerator2" self SelfConstraint Other OtherConstraint)))

(fn `AttachOtherFromSelf`
  (params (Params :type "/Game/Core/Structures/S_ConstraintData Structure"))
  (locals (OtherTrack :type "/Game/Code/Boxes/BP_ConstraintBox Object Reference") (SelfConstraintTrack :type "PhysicsConstraintComponent Object Reference") (OtherConstraintTrack :type "PhysicsConstraintComponent Object Reference"))
  (bind (_constraintowner _self _selfconstraint _other _otherconstraint) (break `/Game/Core/Structures/S_ConstraintData` Params))
  (bind _params (`local.Params`))
  (bind (_constraintowner_2 _self_2 _selfconstraint_2 _other_2 _otherconstraint_2) (break `/Game/Core/Structures/S_ConstraintData` _params))
  (bind _center (`/Game/Code/Boxes/BP_ConstraintBox.Center` (`local.OtherTrack`)))
  (bind _returnvalue (`KismetMathLibrary.ComposeRotators` (`KismetMathLibrary.NegateRotator` (`SceneComponent.RelativeRotation` (`local.OtherConstraintTrack`))) (`/Game/Code/ProjectLibraries/BPML_Global.Opposite Rotator` (`SceneComponent.K2_GetComponentRotation` (`local.SelfConstraintTrack`)))))
  (bind _roota (`self.GetOtherAttachmentPosition` (`SceneComponent.K2_GetComponentLocation` (`local.SelfConstraintTrack`)) (`SceneComponent.K2_GetComponentLocation` (`/Game/Code/Boxes/BP_ConstraintBox.Center` (`local.OtherTrack`))) (`SceneComponent.K2_GetComponentLocation` (`local.OtherConstraintTrack`))))
  (set `local.SelfConstraintTrack` _selfconstraint)
  (set `local.OtherTrack` _other)
  (set `local.OtherConstraintTrack` _otherconstraint)
  (if (not (`BlueprintMapLibrary.Map_Contains` (`self.ConstraintedObjects`) (`local.SelfConstraintTrack`)))
    (`KismetSystemLibrary.PrintString` (`KismetStringLibrary.Concat_StrStr` "Attachment: " (`KismetSystemLibrary.GetDisplayName` self) " -> " (`KismetSystemLibrary.GetDisplayName` (`local.OtherTrack`)) " (" (`|GetEnumeratorNameAsString` _constraintowner) ")"))
    (if (`|EnumEquality` _constraintowner "NewEnumerator0")
      (bind _outhits (`KismetSystemLibrary.BoxTraceMulti` :`Start` _roota :`End` _roota :`HalfSize` (* (`BoxComponent.GetScaledBoxExtent` (`/Game/Code/Boxes/BP_ConstraintBox.CollisionEnforcer` (`local.OtherTrack`))) 0.9) :`Orientation` _returnvalue :`TraceChannel` "TraceTypeQuery1" :`DrawDebugType` "ForDuration" :`bIgnoreSelf` false))
      (bind (_okay _attachments) (`self.GetUnconnectedConnections` _outhits (`local.Params`)))
      (if _okay
        (`|ExecutionSequence`
          (:`then_1`
            (for _array_element _attachments
              (bind _asbp_constraint_box (cast `/Game/Code/Boxes/BP_ConstraintBox` (`ActorComponent.GetOwner` _array_element) :!pure true))
              (`self.AddSoftAttachment` (`local.SelfConstraintTrack`) _asbp_constraint_box _array_element)
              (`self.AddSoftAttachment` _asbp_constraint_box _array_element self (`local.SelfConstraintTrack`))))
          (:`then_2`
            (`SceneComponent.K2_SetWorldRotation` _center _returnvalue false false)
            (`SceneComponent.K2_SetWorldLocation` _center _roota false false))
          (:`then_3`
            (`PhysicsConstraintComponent.SetConstrainedComponents` (`local.SelfConstraintTrack`) (`self.Center`) "None" (`/Game/Code/Boxes/BP_ConstraintBox.Center` (`local.OtherTrack`)) "None")
            (`BlueprintMapLibrary.Map_Add` (`self.ConstraintedObjects`) (`local.SelfConstraintTrack`) _params)
            (`self.AttachOtherFromSelf` _other_2 (make `/Game/Core/Structures/S_ConstraintData` "NewEnumerator1" _other_2 _otherconstraint_2 _self_2 _selfconstraint_2)))))
      (else
        (`BlueprintMapLibrary.Map_Add` (`self.ConstraintedObjects`) (`local.SelfConstraintTrack`) (`local.Params`))))))

(fn `ConnectedTo (Single)`
  (params (B :type "/Game/Code/Boxes/BP_ConstraintBox Object Reference"))
  (returns (bIsConnected :type Boolean))
  (bind _constraintedobjects (`self.ConstraintedObjects`))
  (if (== self B)
    (return true)
    (else
      (bind _keys (`BlueprintMapLibrary.Map_Keys` _constraintedobjects))
      (for _array_element _keys
        (if (== (`.Other_6_3508B1ED7F423598CD240E8C537F5C61` (break `/Game/Core/Structures/S_ConstraintData` (`BlueprintMapLibrary.Map_Find` _constraintedobjects _array_element))) B)
          (return true)))
      (return false))))

(fn `GenerateDefaultPhysicsConstraint`
  (params (bManualAttachment :type Boolean) (RelativeTransform :type "Transform Structure"))
  (returns (Output :type "PhysicsConstraintComponent Object Reference"))
  (bind _returnvalue (`AddComponent|NODE_AddPhysicsConstraintComponent-1` :`bManualAttachment` bManualAttachment :`RelativeTransform` RelativeTransform))
  (`PhysicsConstraintComponent.SetLinearXLimit` _returnvalue "LCM_Locked" 0.0)
  (`PhysicsConstraintComponent.SetLinearYLimit` _returnvalue "LCM_Locked" 0.0)
  (`PhysicsConstraintComponent.SetLinearZLimit` _returnvalue "LCM_Locked" 0.0)
  (`PhysicsConstraintComponent.SetAngularSwing1Limit` _returnvalue "ACM_Locked" 0.0)
  (`PhysicsConstraintComponent.SetAngularSwing2Limit` _returnvalue "ACM_Locked" 0.0)
  (`PhysicsConstraintComponent.SetAngularTwistLimit` _returnvalue "ACM_Locked" 0.0)
  (`SceneComponent.K2_AttachToComponent` _returnvalue (`self.Center`) "None" "KeepRelative" "KeepRelative" "KeepRelative" true)
  (return _returnvalue))

(fn `GetAttachmentHits`
  (returns (OutHit :type "Map of PhysicsConstraintComponent Object Reference to /Game/Core/Structures/S_HitResults Structure") (ReturnValue :type Boolean))
  (locals (HitResults :type "Map of PhysicsConstraintComponent Object Reference to /Game/Core/Structures/S_HitResults Structure") (HitAny :type Boolean))
  (for _array_element (`self.Constraints`)
    (if (not (`BlueprintMapLibrary.Map_Contains` (`self.ConstraintedObjects`) _array_element))
      (bind _returnvalue (`SceneComponent.K2_GetComponentLocation` _array_element))
      (bind (_outhits _returnvalue_2) (`KismetSystemLibrary.SphereTraceMulti` :`Start` _returnvalue :`End` _returnvalue :`Radius` 32.0 :`TraceChannel` "TraceTypeQuery1" :`DrawDebugType` "ForOneFrame" :`DrawTime` 0.1))
      (if _returnvalue_2
        (set `local.HitAny` true)
        (`BlueprintMapLibrary.Map_Add` (`local.HitResults`) _array_element (make `/Game/Core/Structures/S_HitResults` _outhits)))))
  (return (`local.HitResults`) (`local.HitAny`)))

(fn `GetChainCascade`)

(fn `GetNearestOtherConstraint`
  (params (SelfConstraint :type "PhysicsConstraintComponent Object Reference") (Hits :type "/Game/Core/Structures/S_HitResults Structure"))
  (returns (Success :type Boolean) (Actor :type "/Game/Code/Boxes/BP_ConstraintBox Object Reference") (Component :type "PhysicsConstraintComponent Object Reference") (Distance :type "Float (double-precision)"))
  (locals (NearestLength :type "Float (double-precision)") (NearestComponent :type "PhysicsConstraintComponent Object Reference") (FoundAnyNearest :type Boolean) (NearestActor :type "/Game/Code/Boxes/BP_ConstraintBox Object Reference"))
  (bind _value (break `/Game/Core/Structures/S_HitResults` Hits))
  (`/Game/Code/ProjectLibraries/BPML_Global.Assert` (> (`KismetArrayLibrary.Array_Length` _value) 0) "GetNearestOtherConstraint: Passed in empty array"
    (:`then`
      (for _array_element _value
        (bind _asbp_constraint_box (cast `/Game/Code/Boxes/BP_ConstraintBox` (`.HitActor` (`GameplayStatics.BreakHitResult` _array_element))))
        (for _array_element_2 (`/Game/Code/Boxes/BP_ConstraintBox.Constraints` _asbp_constraint_box)
          (bind _returnvalue (`KismetMathLibrary.Vector_Distance` (`SceneComponent.K2_GetComponentLocation` _array_element_2) (`SceneComponent.K2_GetComponentLocation` SelfConstraint)))
          (if (and (or (not (`local.FoundAnyNearest`)) (>= (`local.NearestLength`) _returnvalue)) (not (`BlueprintMapLibrary.Map_Contains` (`/Game/Code/Boxes/BP_ConstraintBox.ConstraintedObjects` _asbp_constraint_box) _array_element_2)))
            (set `local.FoundAnyNearest` true)
            (set `local.NearestComponent` _array_element_2)
            (set `local.NearestLength` _returnvalue)
            (set `local.NearestActor` _asbp_constraint_box))))
      (return (`local.FoundAnyNearest`) (`local.NearestActor`) (`local.NearestComponent`) (`local.NearestLength`)))
    (:`Fail`
      (return false null null 0.0))))

(fn `GetUnconnectedConnections`
  (params (HitResults :type "Array of HitResult Structure") (SafetyParams :type "/Game/Core/Structures/S_ConstraintData Structure"))
  (returns (Okay :type Boolean) (Attachments :type "Array of PhysicsConstraintComponent Object Reference"))
  (locals (SafeAttachments :type "Array of PhysicsConstraintComponent Object Reference"))
  (bind (_constraintowner _self _selfconstraint _other) (break `/Game/Core/Structures/S_ConstraintData` (`local.SafetyParams`)))
  (for _array_element HitResults
    (bind (_bblockinghit _binitialoverlap _time _distance _location _impactpoint _normal _impactnormal _physmat _hitactor _hitcomponent) (`GameplayStatics.BreakHitResult` _array_element))
    (bind _assphere_collision (cast `SphereComponent` _hitcomponent))
    (bind _asbp_constraint_box (cast `/Game/Code/Boxes/BP_ConstraintBox` (`ActorComponent.GetOwner` _assphere_collision)))
    (bind _asphysics_constraint_component (cast `PhysicsConstraintComponent` (`SceneComponent.GetAttachParent` _assphere_collision)))
    (if (and (!= _other _hitactor) (!= _selfconstraint _asphysics_constraint_component))
      (if (not (`BlueprintMapLibrary.Map_Contains` (`/Game/Code/Boxes/BP_ConstraintBox.ConstraintedObjects` _asbp_constraint_box) _asphysics_constraint_component))
        (`KismetArrayLibrary.Array_Add` (`local.SafeAttachments`) _asphysics_constraint_component)
        (else
          (return false)))))
  (return true (`local.SafeAttachments`)))

(fn `UpdateCollisionAttachments`
  (bind _outhit (`self.GetAttachmentHits`))
  (bind _keys (`BlueprintMapLibrary.Map_Keys` _outhit))
  (if (`BlueprintMapLibrary.Map_IsNotEmpty` _outhit)
    (for _array_element _keys
      (bind (_success _actor _component) (`self.GetNearestOtherConstraint` _array_element (`BlueprintMapLibrary.Map_Find` _outhit _array_element)))
      (if _success
        (bind _bisconnected (`self.ConnectedTo (Single)` _actor))
        (if (not _bisconnected)
          (`self.AttachOtherFromSelf` (make `/Game/Core/Structures/S_ConstraintData` "NewEnumerator0" self _array_element _actor _component)))))))

(fn `UserConstructionScript`
  (`TextRenderComponent.K2_SetText` (`self.Display`) (`KismetTextLibrary.Conv_StringToText` (`/Game/Code/ProjectLibraries/BPFL_Global.String To Words` (`|GetEnumeratorNameAsString` (`self.Contents`)))))
  (for _array_element (`self.ConstraintConfig`)
    (bind (_faces _originlineoffset _points) (break `/Game/Core/Structures/S_ConstraintBoxFace` _array_element))
    (for _array_element_2 _faces
      (for _array_element_3 _points
        (bind (_lookvector _direction) (`/Game/Code/ProjectLibraries/BPML_Global.FaceDirection` _array_element_2))
        (bind (_x _y) (`KismetMathLibrary.BreakVector2D` (* _array_element_3 -1.0)))
        (bind _output (`self.GenerateDefaultPhysicsConstraint` false (`KismetMathLibrary.MakeTransform` (+ (* (`KismetMathLibrary.GetRightVector` _direction) _x) (* (`KismetMathLibrary.GetUpVector` _direction) _y) (* _lookvector (`KismetMathLibrary.Conv_DoubleToVector` _originlineoffset))) _direction)))
        (bind _returnvalue (`AddComponent|NODE_AddSphereComponent-0`))
        (`SphereComponent.SetSphereRadius` _returnvalue 32.0 true)
        (`SceneComponent.K2_AttachToComponent` _returnvalue _output "None" "KeepRelative" "KeepRelative" "KeepRelative" true)
        (bind _returnvalue_2 (`AddComponent|NODE_AddArrowComponent-0`))
        (`SceneComponent.K2_AttachToComponent` _returnvalue_2 _output "None" "KeepRelative" "KeepRelative" "KeepRelative" true)))))