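; BP_ConstraintBoxTest is a test box actor that joins itself to touching boxes of the same class with a physics constraint.
; While unconstrained, each Tick runs a tiny debug-drawn sphere trace at its PhysicsConstraint location.
; An unconstrained box it hits gets linked by Cube components, and both cubes ignore PhysicsBody collision.
; Only the hit box's Constrainted flag is set, so the initiator keeps tracing until another box claims it.
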(event `self.ReceiveTick`
  (params (DeltaSeconds :type "Float (single-precision)"))
  (bind _returnvalue (`SceneComponent.K2_GetComponentLocation` (`self.PhysicsConstraint`)))
  (if (not (`self.Constrainted`))
    (bind _outhits (`KismetSystemLibrary.SphereTraceMulti` :`Start` _returnvalue :`End` _returnvalue :`Radius` 1.0 :`TraceChannel` "TraceTypeQuery1" :`DrawDebugType` "ForDuration"))
    (for _array_element _outhits
      (bind _asbp_constraint_box_test (cast `/Game/Code/Boxes/BP_ConstraintBoxTest` (`.HitActor` (`GameplayStatics.BreakHitResult` _array_element))))
      (if (not (`/Game/Code/Boxes/BP_ConstraintBoxTest.Constrainted` _asbp_constraint_box_test))
        (set `/Game/Code/Boxes/BP_ConstraintBoxTest.Constrainted` true _asbp_constraint_box_test)
        (bind _cube (`/Game/Code/Boxes/BP_ConstraintBoxTest.Cube` _asbp_constraint_box_test))
        (`PhysicsConstraintComponent.SetConstrainedComponents` (`self.PhysicsConstraint`) (`self.Cube`) "None" _cube "None")
        (`|ExecutionSequence`
          (:`then_0`
            (`PrimitiveComponent.SetCollisionResponseToChannel` (`self.Cube`) "ECC_PhysicsBody" "ECR_Ignore"))
          (:`then_1`
            (`PrimitiveComponent.SetCollisionResponseToChannel` _cube "ECC_PhysicsBody" "ECR_Ignore")))))))

(event `self.ReceiveBeginPlay`)

(fn `UserConstructionScript`)