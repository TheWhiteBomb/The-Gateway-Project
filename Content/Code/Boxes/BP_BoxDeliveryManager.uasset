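; Manager actor that delivers a new batch of boxes around its location each time NextDay is called.
; NextDay increments the day and attempts 7–9 BP_GWBoxBase spawns at random nearby offsets and yaws, skipping any blocked by collision.
; Each box gets random Size and Contents enum values, excluding the last two content entries, then refreshes its display.
; Debug prints log deliveries, but re-roll the random offset, so logged locations differ from actual ones.
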(event `self.ReceiveBeginPlay`)

(event `self.ReceiveTick`
  (params (DeltaSeconds :type "Float (single-precision)")))

(fn `NextDay`
  (locals (Count :type Integer :default 0))
  (bind _returnvalue (`KismetMathLibrary.RandomFloatInRange` 0.0 6.28))
  (bind _returnvalue_2 (+ (.location (`self.GetTransform`)) (`KismetMathLibrary.MakeVector` (* (`KismetMathLibrary.Sin` _returnvalue) 200.0) (* (`KismetMathLibrary.Cos` _returnvalue) 200.0))))
  (bind _output_get (set `self.Day` (+ (`self.Day`) 1)))
  (`KismetSystemLibrary.PrintString` (`KismetStringLibrary.Concat_StrStr` "[==[ Delivering day '" (`KismetStringLibrary.Conv_IntToString` _output_get) "' of boxes ]==]"))
  (bind _output_get_2 (set `local.Count` (`KismetMathLibrary.RandomIntegerInRange` 7 9)))
  (for _index (range 1 (+ _output_get_2 1))
    (bind _returnvalue_3 (`|SpawnActorFromClass` "/Game/Code/Boxes/Base/BP_GWBoxBase.BP_GWBoxBase_C" (`KismetMathLibrary.MakeTransform` _returnvalue_2 (`KismetMathLibrary.MakeRotator` 0.0 0.0 (`KismetMathLibrary.RandomFloatInRange` 0.0 359.99))) "AdjustIfPossibleButDontSpawnIfColliding" "MultiplyWithRoot" null null))
    (`/Engine/EditorBlueprintResources/StandardMacros.IsValid` _returnvalue_3
      (:`Is Valid`
        (bind _output_get_3 (set `/Game/Code/Boxes/Base/BP_GWBoxBase.Size` (cast `/Game/Core/Enums/E_BagSizes` (`KismetMathLibrary.Conv_IntToByte` (`KismetMathLibrary.RandomInteger` (enumcount `/Game/Core/Enums/E_BagSizes`)))) _returnvalue_3))
        (bind _output_get_4 (set `/Game/Code/Boxes/Base/BP_GWBoxBase.Contents` (cast `/Game/Core/Enums/E_BagType` (`KismetMathLibrary.Conv_IntToByte` (`KismetMathLibrary.RandomInteger` (- (enumcount `/Game/Core/Enums/E_BagType`) 2)))) _returnvalue_3))
        (`/Game/Code/Boxes/Base/BP_GWBoxBase.UpdateDisplay` _returnvalue_3)
        (`KismetSystemLibrary.PrintString` (`KismetStringLibrary.Concat_StrStr` "Spawned Box: \"" (`KismetSystemLibrary.GetDisplayName` _returnvalue_3) " At: { " (`KismetStringLibrary.Conv_VectorToString` _returnvalue_2) "} (#" (`KismetStringLibrary.Conv_IntToString` _index) "/" (`KismetStringLibrary.Conv_IntToString` (`local.Count`)) ")" " Size: " (`|GetEnumeratorNameAsString` _output_get_3) " Contents: " (`|GetEnumeratorNameAsString` _output_get_4))))
      (:`Is Not Valid`
        (`KismetSystemLibrary.PrintString` "Ignored spawning of box!"))))
  (`KismetSystemLibrary.PrintString` "[==[ Box delivery complete ]==]"))

(fn `UserConstructionScript`)