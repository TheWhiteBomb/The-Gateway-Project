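; Box actor that snaps and binds to other BP_BindActors21 boxes when its binder components overlap their HitBox-tagged components.
; Four Binder/Binded overlap events record candidate pairs in OverlappedComponents, then share one loop over that map.
; The first valid pair rotates the cube toward the other's axes via dot-product and quaternion tests, shifts it binder-to-binder and attaches it.
; Processed pairs move into both boxes' ConnectedComponents maps.
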(event `HelloThisIsMyTestEVent`
  (params (OverlappedComponent :type "PrimitiveComponent Object Reference") (OtherActor :type "Actor Object Reference") (OtherComp :type "PrimitiveComponent Object Reference") (OtherBodyIndex :type Integer) (bFromSweep :type Boolean) (SweepResult :type "HitResult Structure (by ref)")))

(event `self.Binder1.OnComponentBeginOverlap`
  (params (OverlappedComponent :type "PrimitiveComponent Object Reference") (OtherActor :type "Actor Object Reference") (OtherComp :type "PrimitiveComponent Object Reference") (OtherBodyIndex :type Integer) (bFromSweep :type Boolean) (SweepResult :type "HitResult Structure (by ref)"))
  (bind _cubemesh (`self.CubeMesh`))
  (bind _cubemesh_2 (`self.CubeMesh`))
  (bind _cubemesh_3 (`self.CubeMesh`))
  (bind _returnvalue (`SceneComponent.GetForwardVector` _cubemesh_2))
  (bind _returnvalue_2 (`SceneComponent.GetUpVector` _cubemesh_2))
  (bind _returnvalue_3 (`SceneComponent.GetRightVector` _cubemesh_2))
  (bind _returnvalue_4 (`SceneComponent.GetUpVector` _cubemesh_3))
  (bind _returnvalue_5 (`SceneComponent.GetRightVector` _cubemesh_3))
  (bind _returnvalue_6 (`SceneComponent.GetForwardVector` _cubemesh))
  (bind _returnvalue_7 (`SceneComponent.GetUpVector` _cubemesh))
  (bind _returnvalue_8 (`SceneComponent.GetRightVector` _cubemesh))
  (`self.BoxOverlapWhileHolding` OverlappedComponent OtherComp)
  (bind (_keypin _valuepin) (`|MapForEach` (`self.OverlappedComponents`) :!label _label)
    (:`then`
      (bind (_asbp_bind_actors_21 _bsuccess) (cast `/Game/Code/Boxes/BP_BindActors21` (`ActorComponent.GetOwner` _valuepin) :!pure true))
      (if (and (`BlueprintMapLibrary.Map_Contains` (`self.ConnectedComponents`) _keypin) _bsuccess)
        _
        (elif (not (`BlueprintMapLibrary.Map_Contains` (`/Game/Code/Boxes/BP_BindActors21.ConnectedComponents` _asbp_bind_actors_21) _valuepin))
          (`|ExecutionSequence`
            (:`then_0`
              (`/Engine/EditorBlueprintResources/StandardMacros.DoOnce` false :!label _label_2
                (:`Completed`
                  (`|ExecutionSequence`
                    (:`then_0`
                      (set `self.ConnectedParent` _asbp_bind_actors_21)
                      (`|ExecutionSequence`
                        (:`then_0`
                          (bind _cubemesh_4 (`/Game/Code/Boxes/BP_BindActors21.CubeMesh` _asbp_bind_actors_21))
                          (bind _returnvalue_9 (`SceneComponent.GetForwardVector` _cubemesh_4))
                          (bind _returnvalue_10 (`KismetMathLibrary.Dot_VectorVector` _returnvalue_9 _returnvalue))
                          (bind _returnvalue_11 (`KismetMathLibrary.Abs` _returnvalue_10))
                          (bind _returnvalue_12 (`KismetMathLibrary.Dot_VectorVector` _returnvalue_9 _returnvalue_2))
                          (bind _returnvalue_13 (`KismetMathLibrary.Abs` _returnvalue_12))
                          (bind _returnvalue_14 (`KismetMathLibrary.Dot_VectorVector` _returnvalue_9 _returnvalue_3))
                          (bind _returnvalue_15 (`KismetMathLibrary.Abs` _returnvalue_14))
                          (bind _returnvalue_16 (`KismetMathLibrary.FMax` _returnvalue_11 _returnvalue_13 _returnvalue_15))
                          (if (== _returnvalue_11 _returnvalue_16)
                            (`SceneComponent.K2_AddWorldRotation` (`self.CubeMesh`) (`KismetMathLibrary.Quat_Rotator` (`KismetMathLibrary.Quat_FindBetweenVectors` (select `bool` (> _returnvalue_10 0.0) :`false` (* _returnvalue -1.0) :`true` _returnvalue) _returnvalue_9)) false false)
                            (elif (== _returnvalue_13 _returnvalue_16)
                              (`SceneComponent.K2_AddWorldRotation` (`self.CubeMesh`) (`KismetMathLibrary.Quat_Rotator` (`KismetMathLibrary.Quat_FindBetweenVectors` (select `bool` (> _returnvalue_12 0.0) :`false` (* _returnvalue_2 -1.0) :`true` _returnvalue_2) _returnvalue_9)) false false)
                              (elif (== _returnvalue_15 _returnvalue_16)
                                (`SceneComponent.K2_AddWorldRotation` (`self.CubeMesh`) (`KismetMathLibrary.Quat_Rotator` (`KismetMathLibrary.Quat_FindBetweenVectors` (select `bool` (> _returnvalue_14 0.0) :`false` (* _returnvalue_3 -1.0) :`true` _returnvalue_3) _returnvalue_9)) false false)))))
                        (:`then_1`
                          (bind _returnvalue_17 (`SceneComponent.GetUpVector` _cubemesh_4))
                          (bind _returnvalue_18 (`KismetMathLibrary.Dot_VectorVector` _returnvalue_17 _returnvalue_17))
                          (bind _returnvalue_19 (`KismetMathLibrary.Abs` _returnvalue_18))
                          (bind _returnvalue_20 (`KismetMathLibrary.Dot_VectorVector` _returnvalue_17 _returnvalue_17))
                          (bind _returnvalue_21 (`KismetMathLibrary.Abs` _returnvalue_20))
                          (bind _returnvalue_22 (`KismetMathLibrary.Dot_VectorVector` _returnvalue_17 _returnvalue_17))
                          (bind _returnvalue_23 (`KismetMathLibrary.Abs` _returnvalue_22))
                          (bind _returnvalue_24 (`KismetMathLibrary.FMax` _returnvalue_19 _returnvalue_21 _returnvalue_23))
                          (if (== _returnvalue_19 _returnvalue_24)
                            (`SceneComponent.K2_AddWorldRotation` (`self.CubeMesh`) (`KismetMathLibrary.Quat_Rotator` (`KismetMathLibrary.Quat_FindBetweenVectors` (select `bool` (> _returnvalue_18 0.0) :`false` (* (`SceneComponent.GetForwardVector` _cubemesh_3) -1.0)) _returnvalue_17)) false false)
                            (elif (== _returnvalue_21 _returnvalue_24)
                              (`SceneComponent.K2_AddWorldRotation` (`self.CubeMesh`) (`KismetMathLibrary.Quat_Rotator` (`KismetMathLibrary.Quat_FindBetweenVectors` (select `bool` (> _returnvalue_20 0.0) :`false` (* _returnvalue_4 -1.0) :`true` _returnvalue_4) _returnvalue_17)) false false)
                              (elif (== _returnvalue_23 _returnvalue_24)
                                (`SceneComponent.K2_AddWorldRotation` (`self.CubeMesh`) (`KismetMathLibrary.Quat_Rotator` (`KismetMathLibrary.Quat_FindBetweenVectors` (select `bool` (> _returnvalue_22 0.0) :`false` (* _returnvalue_5 -1.0) :`true` _returnvalue_5) _returnvalue_17)) false false)))))
                        (:`then_2`
                          (bind _returnvalue_25 (`SceneComponent.GetRightVector` _cubemesh_4))
                          (bind _returnvalue_26 (`KismetMathLibrary.Dot_VectorVector` _returnvalue_6 _returnvalue_25))
                          (bind _returnvalue_27 (`KismetMathLibrary.Abs` _returnvalue_26))
                          (bind _returnvalue_28 (`KismetMathLibrary.Dot_VectorVector` _returnvalue_7 _returnvalue_25))
                          (bind _returnvalue_29 (`KismetMathLibrary.Abs` _returnvalue_28))
                          (bind _returnvalue_30 (`KismetMathLibrary.Dot_VectorVector` _returnvalue_8 _returnvalue_25))
                          (bind _returnvalue_31 (`KismetMathLibrary.Abs` _returnvalue_30))
                          (bind _returnvalue_32 (`KismetMathLibrary.FMax` _returnvalue_27 _returnvalue_29 _returnvalue_31))
                          (if (== _returnvalue_27 _returnvalue_32)
                            (`SceneComponent.K2_AddWorldRotation` (`self.CubeMesh`) (`KismetMathLibrary.Quat_Rotator` (`KismetMathLibrary.Quat_FindBetweenVectors` (select `bool` (> _returnvalue_26 0.0) :`false` (* _returnvalue_6 -1.0)) _returnvalue_25)) false false)
                            (elif (== _returnvalue_29 _returnvalue_32)
                              (`SceneComponent.K2_AddWorldRotation` (`self.CubeMesh`) (`KismetMathLibrary.Quat_Rotator` (`KismetMathLibrary.Quat_FindBetweenVectors` (select `bool` (> _returnvalue_28 0.0) :`false` (* _returnvalue_7 -1.0) :`true` _returnvalue_7) _returnvalue_25)) false false)
                              (elif (== _returnvalue_31 _returnvalue_32)
                                (`SceneComponent.K2_AddWorldRotation` (`self.CubeMesh`) (`KismetMathLibrary.Quat_Rotator` (`KismetMathLibrary.Quat_FindBetweenVectors` (select `bool` (> _returnvalue_30 0.0) :`false` (* _returnvalue_8 -1.0) :`true` _returnvalue_8) _returnvalue_25)) false false)))))))
                    (:`then_1`
                      (`SceneComponent.K2_SetWorldLocation` (`self.CubeMesh`) (+ (`SceneComponent.K2_GetComponentLocation` (`self.CubeMesh`)) (- (`SceneComponent.K2_GetComponentLocation` _valuepin) (`SceneComponent.K2_GetComponentLocation` _keypin))) false true)
                      (`SceneComponent.K2_AttachToComponent` (`self.CubeMesh`) (`/Game/Code/Boxes/BP_BindActors21.CubeMesh` _asbp_bind_actors_21) "None" "KeepWorld" "KeepWorld" "KeepWorld" true))))))
            (:`then_1`
              (`BlueprintMapLibrary.Map_Add` (`self.ConnectedComponents`) _keypin _valuepin)
              (`BlueprintMapLibrary.Map_Remove` (`self.OverlappedComponents`) _keypin)
              (`BlueprintMapLibrary.Map_Remove` (`/Game/Code/Boxes/BP_BindActors21.OverlappedComponents` _asbp_bind_actors_21) _valuepin)
              (`BlueprintMapLibrary.Map_Add` (`/Game/Code/Boxes/BP_BindActors21.ConnectedComponents` _asbp_bind_actors_21) _valuepin _keypin))))))
    (:`CompletedPin`
      (goto _label_2 :!via `Reset`))))

(event `self.Binded1.OnComponentBeginOverlap`
  (params (OverlappedComponent :type "PrimitiveComponent Object Reference") (OtherActor :type "Actor Object Reference") (OtherComp :type "PrimitiveComponent Object Reference") (OtherBodyIndex :type Integer) (bFromSweep :type Boolean) (SweepResult :type "HitResult Structure (by ref)"))
  (`self.BoxOverlapWhileHolding` OverlappedComponent OtherComp)
  (goto _label))

(event `self.Binder2.OnComponentBeginOverlap`
  (params (OverlappedComponent :type "PrimitiveComponent Object Reference") (OtherActor :type "Actor Object Reference") (OtherComp :type "PrimitiveComponent Object Reference") (OtherBodyIndex :type Integer) (bFromSweep :type Boolean) (SweepResult :type "HitResult Structure (by ref)"))
  (`self.BoxOverlapWhileHolding` OverlappedComponent OtherComp)
  (goto _label))

(event `self.Binded2.OnComponentBeginOverlap`
  (params (OverlappedComponent :type "PrimitiveComponent Object Reference") (OtherActor :type "Actor Object Reference") (OtherComp :type "PrimitiveComponent Object Reference") (OtherBodyIndex :type Integer) (bFromSweep :type Boolean) (SweepResult :type "HitResult Structure (by ref)"))
  (`self.BoxOverlapWhileHolding` OverlappedComponent OtherComp)
  (goto _label))

(fn `BoxOverlapWhileHolding`
  (params (`Overlapped Comp` :type "PrimitiveComponent Object Reference") (`Other Comp` :type "PrimitiveComponent Object Reference"))
  (bind (_asbp_bind_actors_21 _bsuccess) (cast `/Game/Code/Boxes/BP_BindActors21` (`ActorComponent.GetOwner` `Other Comp`) :!pure true))
  (if (and (`KismetArrayLibrary.Array_Contains` (`ActorComponent.ComponentTags` `Other Comp`) "HitBox") _bsuccess (!= `Other Comp` self))
    (if (not (`BlueprintMapLibrary.Map_Contains` (`/Game/Code/Boxes/BP_BindActors21.ConnectedComponents` _asbp_bind_actors_21) `Other Comp`))
      (`BlueprintMapLibrary.Map_Add` (`self.OverlappedComponents`) `Overlapped Comp` `Other Comp`))))

(fn `UserConstructionScript`)