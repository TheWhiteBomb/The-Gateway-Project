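; BP_GroupManager is an actor that represents a group of connected, grabbable boxes and handles dissolving it.
; FullReset syncs each box's held state from its GrabComponent, clears its attached actors, primitives and group reference, then destroys the manager.
; Before destruction, a second pass teleports each cube mesh to its current location.
; DestroyConstraint separately removes a given constraint component; the event graph is empty.
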(event `self.ReceiveTick`
  (params (DeltaSeconds :type "Float (single-precision)")))

(fn `DestroyConstraint`
  (params (Constraint :type "PhysicsConstraintComponent Object Reference"))
  (`ActorComponent.K2_DestroyComponent` Constraint)
  (return))

(fn `Full reset`
  (for _array_element (`self.ConnectedBoxes`)
    (set `/Game/Code/Boxes/Base/BP_BindActors.IS Held` (`/Game/VRTemplate/Blueprints/GrabComponent.bIsHeld` (`/Game/Code/Boxes/Base/BP_BindActors.GrabComponent` _array_element)) _array_element)
    (`KismetArrayLibrary.Array_Clear` (`/Game/Code/Boxes/Base/BP_BindActors.AttatchedActors` _array_element))
    (`BlueprintMapLibrary.Map_Clear` (`/Game/Code/Boxes/Base/BP_BindActors.AttatchedPrimitives` _array_element))
    (set `/Game/Code/Boxes/Base/BP_BindActors.BindGroup` null _array_element))
  (for _array_element_2 (`self.ConnectedBoxes`)
    (`SceneComponent.K2_SetWorldLocation` (`/Game/Code/Boxes/Base/BP_BindActors.CubeMesh` _array_element_2) (`SceneComponent.K2_GetComponentLocation` (`/Game/Code/Boxes/Base/BP_BindActors.CubeMesh` _array_element_2)) false true))
  (`self.K2_DestroyActor`))

(fn `UserConstructionScript`)