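; Grabbable cube box that snaps to other BP_BindActors boxes and binds to them with physics constraints.
; At BeginPlay it spawns "Binder" spheres at mesh sockets, whose overlaps record pairs and notify GatewayGameMode.
; On release, SnapToCube can shift the mesh, rotate it toward the target's closest axes using dot products, and add constraints.
; Hand-overlap logic destroys constraints, but depends on AttatchedComponents, which nothing here fills; end-overlap handling is unfinished.
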(event `self.GrabComponent.OnDropped`
  (set `self.IsHeld` false)
  (if (`self.SnapOnRelease`)
    (`self.SnapToCube` (`self.SnapTwin`))))

(event `self.GrabComponent.OnGrabbed`
  (set `self.IsHeld` true))

(event `self.ReceiveTick`
  (params (DeltaSeconds :type "Float (single-precision)"))
  (`self.K2_SetActorTransform` (`SceneComponent.K2_GetComponentToWorld` (`self.CubeMesh`)))
  (`SceneComponent.K2_SetWorldTransform` (`self.CubeMesh`) (`self.GetTransform`) false false))

(event `BindActorsBegin`
  (params (OverlappedComponent :type "PrimitiveComponent Object Reference") (OtherActor :type "Actor Object Reference") (OtherComp :type "PrimitiveComponent Object Reference") (OtherBodyIndex :type Integer) (bFromSweep :type Boolean) (SweepResult :type "HitResult Structure (by ref)"))
  (`self.SetOverlappingBoxCollissions` OverlappedComponent OtherActor OtherComp))

(event `BindActorsEnd`
  (params (OverlappedComponent :type "PrimitiveComponent Object Reference") (OtherActor :type "Actor Object Reference") (OtherComp :type "PrimitiveComponent Object Reference") (OtherBodyIndex :type Integer)))

(event `self.ReceiveBeginPlay`
  (`KismetSystemLibrary.DelayUntilNextTick`)
  (`self.CreateCollisions`)
  (bind _asgateway_game_mode (cast `/Game/Code/Persistent/GatewayGameMode` (`GameplayStatics.GetGameMode`)))
  (set `self.GatewayGameMode` _asgateway_game_mode))

(fn `CreateCollisions`
  (for _array_element (`SceneComponent.GetAllSocketNames` (`self.CubeMesh`))
    (bind _returnvalue (`AddComponent|NODE_AddSphereComponent-1`))
    (`SceneComponent.K2_SetWorldLocation` _returnvalue (`SceneComponent.GetSocketLocation` (`self.CubeMesh`) _array_element) false true)
    (`SceneComponent.K2_AttachToComponent` _returnvalue (`self.CubeMesh`) _array_element "KeepWorld" "KeepWorld" "KeepWorld" true)
    (`/Game/Code/ProjectLibraries/BPML_General.AddComponentTag` _returnvalue "Binder")
    (add `PrimitiveComponent.OnComponentBeginOverlap` _returnvalue (`|CreateDelegate` :!event `BindActorsBegin`))
    (add `PrimitiveComponent.OnComponentEndOverlap` _returnvalue (`|CreateDelegate` :!event `BindActorsEnd`))))

(fn `RemoveOverlappingCollissions`
  (params (SourceComp :type "PrimitiveComponent Object Reference") (Target :type "Actor Object Reference") (TargetComp :type "PrimitiveComponent Object Reference"))
  (bind _keys (`BlueprintMapLibrary.Map_Keys` (`self.ConnectedComponents`)))
  (if (`KismetArrayLibrary.Array_Contains` _keys (`local.SourceComp`))
    _))

(fn `SetEndOverlap`
  (params (Key :type "PrimitiveComponent Object Reference (by ref)") (InputPin :type "PrimitiveComponent Object Reference"))
  (bind (_asbp_bind_actors _bsuccess) (cast `/Game/Code/Boxes/Base/BP_BindActors` (`ActorComponent.GetOwner` InputPin) :!pure true))
  (if (and (`KismetArrayLibrary.Array_Contains` (`ActorComponent.ComponentTags` InputPin) "HitBox") (!= null self))
    (if (and _bsuccess (not (`KismetArrayLibrary.Array_Contains` (`/Game/Code/Boxes/Base/BP_BindActors.AttatchedComponents` _asbp_bind_actors))))
      (`BlueprintMapLibrary.Map_Remove` (`self.OverlappedComponents`) Key))))

(fn `SetOverlappingBoxCollissions`
  (params (SourceComp :type "PrimitiveComponent Object Reference") (Target :type "Actor Object Reference") (TargetComp :type "PrimitiveComponent Object Reference"))
  (bind _targetcomp (`local.TargetComp`))
  (bind _asbp_shared_pawn (cast `/Game/Code/ZeroGravity/BP_SharedPawn` (`GameplayStatics.GetPlayerPawn` 0) :!pure true))
  (if (== (`local.Target`) _asbp_shared_pawn)
    (if (or (== (`/Game/Code/ZeroGravity/BP_SharedPawn.HandLeft` _asbp_shared_pawn) _targetcomp) (== _targetcomp (`/Game/Code/ZeroGravity/BP_SharedPawn.HandRight` _asbp_shared_pawn)))
      (if (not (`KismetArrayLibrary.Array_IsEmpty` (`self.AttatchedComponents`)))
        (bind _keypin (`|MapForEach` (`self.ConnectedComponents`) :!label _label)
          (:`then`
            (if (== _keypin (`local.SourceComp`))
              (bind (_value _returnvalue) (`BlueprintMapLibrary.Map_Find` (`self.ConstraintMap`) _keypin))
              (if _returnvalue
                (`ActorComponent.K2_DestroyComponent` _value)
                (`BlueprintMapLibrary.Map_Remove` (`self.ConstraintMap`) _keypin))
              (`KismetArrayLibrary.Array_RemoveItem` (`self.AttatchedComponents`))
              (goto _label :!via `BreakPin`))))))
    (else
      (bind _keys (`BlueprintMapLibrary.Map_Keys` (`self.ConnectedComponents`)))
      (if (not (`KismetArrayLibrary.Array_Contains` _keys (`local.SourceComp`)))
        (if (`KismetArrayLibrary.Array_Contains` (`ActorComponent.ComponentTags` (`local.TargetComp`)) "Binder")
          (if (`.bSuccess` (cast `/Game/Code/Boxes/Base/BP_BindActors` (`local.Target`) :!pure true))
            (`BlueprintMapLibrary.Map_Add` (`self.OverlappedBoxCollissions`) (`local.SourceComp`) (`local.TargetComp`))
            (`/Game/Code/Persistent/GatewayGameMode.TellBoxesToConnect` (`self.GatewayGameMode`) self (cast `/Game/Code/Boxes/Base/BP_BindActors` (`local.Target`) :!pure true))
            (elif (`.bSuccess` (cast `/Game/Code/Persistent/BP_ModuleBase` (`local.Target`) :!pure true))
              _)))))))

(fn `SetOverlappingComponents`
  (params (`Overlapped Comp` :type "PrimitiveComponent Object Reference") (`Other Actor` :type "Actor Object Reference") (`Other Comp` :type "PrimitiveComponent Object Reference"))
  (bind _constraintmap (`self.ConstraintMap`))
  (bind _asbp_shared_pawn (cast `/Game/Code/ZeroGravity/BP_SharedPawn` (`GameplayStatics.GetPlayerPawn` 0) :!pure true))
  (if (== `Other Actor` _asbp_shared_pawn)
    (if (or (== (`/Game/Code/ZeroGravity/BP_SharedPawn.HandLeft` _asbp_shared_pawn) `Other Comp`) (== `Other Comp` (`/Game/Code/ZeroGravity/BP_SharedPawn.HandRight` _asbp_shared_pawn)))
      (if (not (`KismetArrayLibrary.Array_IsEmpty` (`self.AttatchedComponents`)))
        (for _array_element (`self.AttatchedComponents`)
          (if (== _array_element `Overlapped Comp`)
            (bind (_value _returnvalue) (`BlueprintMapLibrary.Map_Find` _constraintmap _array_element))
            (if _returnvalue
              (`ActorComponent.K2_DestroyComponent` _value)
              (`BlueprintMapLibrary.Map_Remove` _constraintmap _array_element))
            (`KismetArrayLibrary.Array_RemoveItem` (`self.AttatchedComponents`) _array_element)
            (break)))))
    (elif (and (`KismetArrayLibrary.Array_Contains` (`ActorComponent.ComponentTags` `Other Comp`) "HitBox") (!= `Other Actor` self))
      (if (`.bSuccess` (cast `/Game/Code/Boxes/Base/BP_BindActors` (`ActorComponent.GetOwner` `Other Comp`) :!pure true))
        (`BlueprintMapLibrary.Map_Add` (`self.OverlappedComponents`) `Overlapped Comp` `Other Comp`)))))

(fn `SetRotation`
  (params (`Other Actor` :type "/Game/Code/Boxes/Base/BP_BindActors Object Reference"))
  (bind _cubemesh (`/Game/Code/Boxes/Base/BP_BindActors.CubeMesh` `Other Actor`))
  (bind _cubemesh_2 (`self.CubeMesh`))
  (bind _cubemesh_3 (`self.CubeMesh`))
  (bind _cubemesh_4 (`self.CubeMesh`))
  (bind _returnvalue (`SceneComponent.GetUpVector` _cubemesh))
  (bind _returnvalue_2 (`SceneComponent.GetRightVector` _cubemesh))
  (bind _returnvalue_3 (`SceneComponent.GetForwardVector` _cubemesh_3))
  (bind _returnvalue_4 (`SceneComponent.GetUpVector` _cubemesh_3))
  (bind _returnvalue_5 (`SceneComponent.GetRightVector` _cubemesh_3))
  (bind _returnvalue_6 (`SceneComponent.GetUpVector` _cubemesh_4))
  (bind _returnvalue_7 (`SceneComponent.GetRightVector` _cubemesh_4))
  (bind _returnvalue_8 (`SceneComponent.GetForwardVector` _cubemesh))
  (bind _returnvalue_9 (`SceneComponent.GetForwardVector` _cubemesh_2))
  (bind _returnvalue_10 (`SceneComponent.GetUpVector` _cubemesh_2))
  (bind _returnvalue_11 (`SceneComponent.GetRightVector` _cubemesh_2))
  (bind _returnvalue_12 (`KismetMathLibrary.Dot_VectorVector` _returnvalue_8 _returnvalue_3))
  (bind _returnvalue_13 (`KismetMathLibrary.Dot_VectorVector` _returnvalue_8 _returnvalue_4))
  (bind _returnvalue_14 (`KismetMathLibrary.Dot_VectorVector` _returnvalue_8 _returnvalue_5))
  (bind _returnvalue_15 (`KismetMathLibrary.Dot_VectorVector` _returnvalue _returnvalue))
  (bind _returnvalue_16 (`KismetMathLibrary.Dot_VectorVector` _returnvalue _returnvalue))
  (bind _returnvalue_17 (`KismetMathLibrary.Dot_VectorVector` _returnvalue _returnvalue))
  (bind _returnvalue_18 (`KismetMathLibrary.Dot_VectorVector` _returnvalue_9 _returnvalue_2))
  (bind _returnvalue_19 (`KismetMathLibrary.Dot_VectorVector` _returnvalue_10 _returnvalue_2))
  (bind _returnvalue_20 (`KismetMathLibrary.Dot_VectorVector` _returnvalue_11 _returnvalue_2))
  (bind _returnvalue_21 (`KismetMathLibrary.Abs` _returnvalue_12))
  (bind _returnvalue_22 (`KismetMathLibrary.Abs` _returnvalue_13))
  (bind _returnvalue_23 (`KismetMathLibrary.Abs` _returnvalue_14))
  (bind _returnvalue_24 (`KismetMathLibrary.Abs` _returnvalue_15))
  (bind _returnvalue_25 (`KismetMathLibrary.Abs` _returnvalue_16))
  (bind _returnvalue_26 (`KismetMathLibrary.Abs` _returnvalue_17))
  (bind _returnvalue_27 (`KismetMathLibrary.Abs` _returnvalue_18))
  (bind _returnvalue_28 (`KismetMathLibrary.Abs` _returnvalue_19))
  (bind _returnvalue_29 (`KismetMathLibrary.Abs` _returnvalue_20))
  (bind _returnvalue_30 (`KismetMathLibrary.FMax` _returnvalue_27 _returnvalue_28 _returnvalue_29))
  (bind _returnvalue_31 (`KismetMathLibrary.FMax` _returnvalue_21 _returnvalue_22 _returnvalue_23))
  (bind _returnvalue_32 (`KismetMathLibrary.FMax` _returnvalue_24 _returnvalue_25 _returnvalue_26))
  (`|ExecutionSequence`
    (:`then_0`
      _)
    (:`then_1`
      _))
  (`|ExecutionSequence`
    (:`then_0`
      (if (== _returnvalue_21 _returnvalue_31)
        (`SceneComponent.K2_AddWorldRotation` (`self.CubeMesh`) (`KismetMathLibrary.Quat_Rotator` (`KismetMathLibrary.Quat_FindBetweenVectors` (select `bool` (> _returnvalue_12 0.0) :`false` (* _returnvalue_3 -1.0) :`true` _returnvalue_3) _returnvalue_8)) false false)
        (elif (== _returnvalue_22 _returnvalue_31)
          (`SceneComponent.K2_AddWorldRotation` (`self.CubeMesh`) (`KismetMathLibrary.Quat_Rotator` (`KismetMathLibrary.Quat_FindBetweenVectors` (select `bool` (> _returnvalue_13 0.0) :`false` (* _returnvalue_4 -1.0) :`true` _returnvalue_4) _returnvalue_8)) false false)
          (elif (== _returnvalue_23 _returnvalue_31)
            (`SceneComponent.K2_AddWorldRotation` (`self.CubeMesh`) (`KismetMathLibrary.Quat_Rotator` (`KismetMathLibrary.Quat_FindBetweenVectors` (select `bool` (> _returnvalue_14 0.0) :`false` (* _returnvalue_5 -1.0) :`true` _returnvalue_5) _returnvalue_8)) false false)))))
    (:`then_1`
      (if (== _returnvalue_24 _returnvalue_32)
        (`SceneComponent.K2_AddWorldRotation` (`self.CubeMesh`) (`KismetMathLibrary.Quat_Rotator` (`KismetMathLibrary.Quat_FindBetweenVectors` (select `bool` (> _returnvalue_15 0.0) :`false` (* (`SceneComponent.GetForwardVector` _cubemesh_4) -1.0)) _returnvalue)) false false)
        (elif (== _returnvalue_25 _returnvalue_32)
          (`SceneComponent.K2_AddWorldRotation` (`self.CubeMesh`) (`KismetMathLibrary.Quat_Rotator` (`KismetMathLibrary.Quat_FindBetweenVectors` (select `bool` (> _returnvalue_16 0.0) :`false` (* _returnvalue_6 -1.0) :`true` _returnvalue_6) _returnvalue)) false false)
          (elif (== _returnvalue_26 _returnvalue_32)
            (`SceneComponent.K2_AddWorldRotation` (`self.CubeMesh`) (`KismetMathLibrary.Quat_Rotator` (`KismetMathLibrary.Quat_FindBetweenVectors` (select `bool` (> _returnvalue_17 0.0) :`false` (* _returnvalue_7 -1.0) :`true` _returnvalue_7) _returnvalue)) false false)))))
    (:`then_2`
      (if (== _returnvalue_27 _returnvalue_30)
        (`SceneComponent.K2_AddWorldRotation` (`self.CubeMesh`) (`KismetMathLibrary.Quat_Rotator` (`KismetMathLibrary.Quat_FindBetweenVectors` (select `bool` (> _returnvalue_18 0.0) :`false` (* _returnvalue_9 -1.0)) _returnvalue_2)) false false)
        (elif (== _returnvalue_28 _returnvalue_30)
          (`SceneComponent.K2_AddWorldRotation` (`self.CubeMesh`) (`KismetMathLibrary.Quat_Rotator` (`KismetMathLibrary.Quat_FindBetweenVectors` (select `bool` (> _returnvalue_19 0.0) :`false` (* _returnvalue_10 -1.0) :`true` _returnvalue_10) _returnvalue_2)) false false)
          (elif (== _returnvalue_29 _returnvalue_30)
            (`SceneComponent.K2_AddWorldRotation` (`self.CubeMesh`) (`KismetMathLibrary.Quat_Rotator` (`KismetMathLibrary.Quat_FindBetweenVectors` (select `bool` (> _returnvalue_20 0.0) :`false` (* _returnvalue_11 -1.0) :`true` _returnvalue_11) _returnvalue_2)) false false)))))))

(fn `SnapToCube`
  (params (Target :type "/Game/Code/Boxes/Base/BP_BindActors Object Reference"))
  (bind (_keypin _valuepin) (`|MapForEach` (`self.OverlappedBoxCollissions`))
    (:`then`
      (`SceneComponent.K2_SetWorldLocation` (`self.CubeMesh`) (+ (`SceneComponent.K2_GetComponentLocation` (`self.CubeMesh`)) (- (`SceneComponent.K2_GetComponentLocation` _keypin) (`SceneComponent.K2_GetComponentLocation` _valuepin))) false false)
      (`self.SetRotation` (`local.Target`))
      (bind _returnvalue (`AddComponent|NODE_AddPhysicsConstraintComponent-2` :`bManualAttachment` true :`RelativeTransform` (`KismetMathLibrary.MakeTransform` (`SceneComponent.K2_GetComponentLocation` _keypin) (`SceneComponent.K2_GetComponentRotation` _keypin))))
      (set `self.Constraint` _returnvalue)
      (`PhysicsConstraintComponent.SetConstrainedComponents` (`self.Constraint`) (`self.CubeMesh`) "None" (`/Game/Code/Boxes/Base/BP_BindActors.CubeMesh` (`local.Target`)) "None")
      (`BlueprintMapLibrary.Map_Add` (`self.ConnectedComponents`) _keypin _valuepin)
      (`BlueprintMapLibrary.Map_Add` (`self.ConstraintMap`) _keypin (`self.Constraint`))
      (`BlueprintMapLibrary.Map_Remove` (`self.OverlappedBoxCollissions`) _keypin))))

(fn `UserConstructionScript`)