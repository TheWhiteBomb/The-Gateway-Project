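; BP_GWBoxBase is a base box actor with a text label naming its contents and a cube mesh matching its size.
; The construction script calls UpdateDisplay, which colors the label, converts the Contents enum name into spaced words for its text, and selects one of four static meshes from the Size value.
; The event graph holds only disabled placeholder events, so it adds no runtime behavior.
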(fn `UpdateDisplay`
  (bind _label (`self.Label`))
  (`TextRenderComponent.SetTextRenderColor` _label (`self.LabelColor`))
  (`TextRenderComponent.K2_SetText` _label (`KismetTextLibrary.Conv_StringToText` (`/Game/Code/ProjectLibraries/BPFL_Global.String To Words` (`|GetEnumeratorNameAsString` (`self.Contents`)))))
  (`StaticMeshComponent.SetStaticMesh` (`self.CubeMesh`) (select `/Game/Core/Enums/E_BagSizes` (`self.Size`) :`NewEnumerator0` "/Game/ArtAndMeshes/Boxes/SM_box1.SM_box1" :`NewEnumerator2` "/Game/ArtAndMeshes/Boxes/SM_box2.SM_box2" :`NewEnumerator3` "/Game/ArtAndMeshes/Boxes/SM_box4.SM_box4" :`NewEnumerator4` "/Game/ArtAndMeshes/Boxes/SM_box6.SM_box6" :!type "StaticMesh Object Reference")))

(fn `UserConstructionScript`
  (`self.UpdateDisplay`)
  (`parent.UserConstructionScript`))