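; Rocket launch sequence actor that moves the rocket upward and provides exhaust effects and a startup camera shake.
; BeginPlay caches the rocket's start transform and creates a hidden Niagara exhaust component for each socket, toggled through SetNiagaraEnabled.
; SetLaunch maps a supplied time to a delayed quartic vertical rise and a random CameraOffset that fades as time advances.
; Tick is empty, so the sequence relies on external calls.
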(event `self.ReceiveBeginPlay`
  (set `self.Start` (`SceneComponent.GetRelativeTransform` (`self.Rocket`)))
  (for _array_element (`SceneComponent.GetAllSocketNames` (`self.Rocket`))
    (bind _returnvalue (`AddComponent|NODE_AddNiagaraComponent-1` :`RelativeTransform` (`KismetMathLibrary.MakeTransform` (- (.location (`self.GetTransform`)) (`SceneComponent.GetSocketLocation` (`self.Rocket`) _array_element)))))
    (`NiagaraComponent.SetAsset` _returnvalue "/Game/ArtAndMeshes/Launching/Special_Effects/NS_RocketExhust.NS_RocketExhust" true)
    (`NiagaraComponent.SetRenderingEnabled` _returnvalue false)
    (`SceneComponent.SetVisibility` _returnvalue false true)
    (`KismetArrayLibrary.Array_Add` (`self.NiagaraSystems`) _returnvalue)))

(fn `SetLaunch`
  (params (Time :type "Float (double-precision)"))
  (if (!= Time 0.0)
    (`SceneComponent.K2_SetRelativeLocation` (`self.Rocket`) (+ (.location (`self.Start`)) (`KismetMathLibrary.MakeVector` 0.0 0.0 (* (`KismetMathLibrary.MultiplyMultiply_FloatFloat` (`KismetMathLibrary.FClamp` (/ (- Time 1.0) 10.0)) 4.0) 30000.0))) false true)
    (set `self.CameraOffset` (* (`/Game/Code/ProjectLibraries/BPML_Global.InvertUnit` (`KismetMathLibrary.FClamp` (/ Time 8.0))) (`KismetMathLibrary.MakeVector` (`KismetMathLibrary.RandomFloat`) (`KismetMathLibrary.RandomFloat`) (`KismetMathLibrary.RandomFloat`)) (`self.StartupShake`)))
    (else
      (`SceneComponent.K2_SetRelativeLocation` (`self.Rocket`) (.location (`self.Start`)) false true))))

(fn `SetNiagaraEnabled`
  (params (bInRenderingEnabled :type Boolean))
  (for _array_element (`self.NiagaraSystems`)
    (`NiagaraComponent.SetRenderingEnabled` _array_element bInRenderingEnabled)
    (`SceneComponent.SetVisibility` _array_element bInRenderingEnabled true)))

(fn `UserConstructionScript`)