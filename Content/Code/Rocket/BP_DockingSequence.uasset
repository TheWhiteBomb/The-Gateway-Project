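; Rocket docking sequence actor that animates a Module component sliding along local X into its starting position.
; BeginPlay caches that relative location, and SetDocking sets the module's offset from the elapsed time passed in as Duration, with no Tick of its own.
; A fifth-power ease-out slows the approach, and a squared-decay random jitter near the end adds a contact shake.
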(event `self.ReceiveBeginPlay`
  (set `self.StartPosition` (`SceneComponent.RelativeLocation` (`self.Module`))))

(fn `SetDocking`
  (params (Duration :type "Float (double-precision)"))
  (bind _returnvalue (- Duration 7.0))
  (`SceneComponent.K2_SetRelativeLocation` (`self.Module`) (+ (`self.StartPosition`) (`KismetMathLibrary.MakeVector` (* (`KismetMathLibrary.MultiplyMultiply_FloatFloat` (`KismetMathLibrary.FClamp` (`/Game/Code/ProjectLibraries/BPML_Global.InvertUnit` (/ Duration 8.0))) 5.0) 200.0)) (select `bool` (> _returnvalue 0.0) :`true` (* (* (`KismetMathLibrary.MultiplyMultiply_FloatFloat` (`KismetMathLibrary.FClamp` (`/Game/Code/ProjectLibraries/BPML_Global.InvertUnit` _returnvalue)) 2.0) 2.0) (`KismetMathLibrary.MakeVector` (`KismetMathLibrary.RandomFloat`) (`KismetMathLibrary.RandomFloat`) (`KismetMathLibrary.RandomFloat`))))) false false))

(fn `UserConstructionScript`)