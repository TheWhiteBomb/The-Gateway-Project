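; Controller that plays the rocket cinematic, running a launch sequence and then a docking sequence once Start is called.
; Tick advances a timer that scrubs BP_LaunchingSequence for ten seconds, then BP_DockingSequence, moving a SceneCapture2D to the active shot's camera with its own FOV.
; Each sequence's shake offset drives camera displacement and controller haptics, while a material parameter collection dips screen brightness to hide the cut.
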(event `self.ReceiveBeginPlay`
  (set `self.LaunchStarted` false)
  (bind _outactors (`GameplayStatics.GetAllActorsOfClass` "/Game/Code/Rocket/BP_LaunchingSequence.BP_LaunchingSequence_C"))
  (set `self.LaunchSequence` (`|GetArrayItem` _outactors))
  (set `self.Sequence` 0.0)
  (bind _outactors_2 (`GameplayStatics.GetAllActorsOfClass` "/Game/Code/Rocket/BP_DockingSequence.BP_DockingSequence_C"))
  (set `self.DockingSequence` (`|GetArrayItem` _outactors_2))
  (bind _outactors_3 (`GameplayStatics.GetAllActorsOfClass` "/Script/Engine.SceneCapture2D"))
  (set `self.SceneCapture` (`|GetArrayItem` _outactors_3))
  (`KismetSystemLibrary.DelayUntilNextTick`)
  (`/Game/Code/Rocket/BP_LaunchingSequence.SetNiagaraEnabled` (`self.LaunchSequence`) false))

(event `self.ReceiveTick`
  (params (DeltaSeconds :type "Float (single-precision)"))
  (bind _returnvalue (`GameplayStatics.GetPlayerController` 0))
  (bind _sequence (`self.Sequence`))
  (bind _scenecapture (`self.SceneCapture`))
  (bind _launchsequence (`self.LaunchSequence`))
  (bind _dockingsequence (`self.DockingSequence`))
  (bind _scenecapture_2 (`self.SceneCapture`))
  (bind _shakeoffset (`/Game/Code/Rocket/BP_DockingSequence.ShakeOffset` _dockingsequence))
  (bind _cameraoffset (`/Game/Code/Rocket/BP_LaunchingSequence.CameraOffset` _launchsequence))
  (if (`self.LaunchStarted`)
    (bind _output_get (set `self.Sequence` (+ DeltaSeconds (`self.Sequence`))))
    (`KismetMaterialLibrary.SetScalarParameterValue` "/Game/Code/Rocket/CameraCubes/MPC_ScreenBrightness.MPC_ScreenBrightness" "Brightness" (`/Game/Code/ProjectLibraries/BPML_Global.Smoothstep` 0.0 1.0 (`KismetMathLibrary.FClamp` (`KismetMathLibrary.Abs` (- _output_get 10.0)))))
    (else
      (set `self.Sequence` 0.0)))
  (if (>= _sequence 10.0)
    (`/Game/Code/Rocket/BP_DockingSequence.SetDocking` _dockingsequence (- _sequence 10.0))
    (`PlayerController.SetHapticsByValue` _returnvalue 2.0 (/ (`KismetMathLibrary.VSize` _shakeoffset) 2.0) "AnyHand")
    (`self.K2_SetActorTransform` _scenecapture (`KismetMathLibrary.MakeTransform` (+ _shakeoffset (.location (`SceneComponent.K2_GetComponentToWorld` (`/Game/Code/Rocket/BP_DockingSequence.CameraLocation` _dockingsequence)))) (.rotation (`SceneComponent.K2_GetComponentToWorld` (`/Game/Code/Rocket/BP_DockingSequence.CameraLocation` _dockingsequence))) (.scale (`SceneComponent.K2_GetComponentToWorld` (`/Game/Code/Rocket/BP_DockingSequence.CameraLocation` _dockingsequence)))) false false)
    (set `SceneCaptureComponent2D.FOVAngle` 120.0 (`SceneCapture2D.CaptureComponent2D` _scenecapture))
    (else
      (`/Game/Code/Rocket/BP_LaunchingSequence.SetLaunch` _launchsequence _sequence)
      (`PlayerController.SetHapticsByValue` _returnvalue 2.0 (/ (`KismetMathLibrary.VSize` _cameraoffset) 150.0) "AnyHand")
      (`self.K2_SetActorTransform` _scenecapture_2 (`KismetMathLibrary.MakeTransform` (+ (.location (`SceneComponent.K2_GetComponentToWorld` (`/Game/Code/Rocket/BP_LaunchingSequence.CameraLocation` _launchsequence))) _cameraoffset) (.rotation (`SceneComponent.K2_GetComponentToWorld` (`/Game/Code/Rocket/BP_LaunchingSequence.CameraLocation` _launchsequence))) (.scale (`SceneComponent.K2_GetComponentToWorld` (`/Game/Code/Rocket/BP_LaunchingSequence.CameraLocation` _launchsequence)))) false false)
      (set `SceneCaptureComponent2D.FOVAngle` 32.720001 (`SceneCapture2D.CaptureComponent2D` _scenecapture_2)))))

(fn `Start`
  (if (not (`self.LaunchStarted`))
    (set `self.LaunchStarted` true)
    (`/Game/Code/Rocket/BP_LaunchingSequence.SetNiagaraEnabled` (`self.LaunchSequence`) true)))

(fn `UserConstructionScript`)