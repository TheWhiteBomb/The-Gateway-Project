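; Base Blueprint for a bag slot that highlights when a bag of the matching size overlaps its snap box.
; The construction script sizes the box from BoxSize and hides the highlight.
; Unless BringIn is set, begin overlap compares size enums, then records the bag and sets HighlightedSlot and BagOverlapping on PC_Gateway; end overlap clears the highlight and flag.
; Helper functions hide the highlight or toggle its collision; RemoveBox is an empty stub.
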(event Custom|OnComponentBeginOverlap_Event
  (params (OverlappedComponent :type Primitive%20Component%20Object%20Reference) (OtherActor :type Actor%20Object%20Reference) (OtherComp :type Primitive%20Component%20Object%20Reference) (OtherBodyIndex :type Integer) (bFromSweep :type Boolean) (SweepResult :type Hit%20Result%20Structure%20%28by%20ref%29))
  ;[1 1 1] tells if a slot is already overlapping with the box, and checks if the slot already has a box in it
  (if (not (Variables|Default|Getbring_In))
    (if (Variables|/Game/Core/PC_Gateway.PC_Gateway_C|GetBagOverlapping (.AsPC%20Gateway (Utilities|Casting|CastToPC_Gateway (Game|GetPlayerController 0))))
      ;[1 1 1] replaces other box as the box it's colliding with
      (Utilities|Casting|CastToBP_LockingParent (Variables|Default|GetBoxHit))
      (Rendering|SetVisibility (Variables|Default|GetHilight) false false))
    ;[1 1 1] Checks if the slot is the right size for the box
    (bind _asbp_bag_parent (Utilities|Casting|CastToBP_BagParent OtherActor))
    (if (|(BSizeEnum==SlotSizeEnum) (Variables|/Game/Code/Bags_And_Locking/Bags/BP_BagParent.BP_BagParent_C|Getenum _asbp_bag_parent) (Variables|Default|GetBagSizeEnum))
      ;[1 1 1] If it is the right slot, the player controller sets the actor variable "hilighted box" so that the bag can tell witch box it's colliding with
      (Variables|/Game/Core/PC_Gateway.PC_Gateway_C|SetHighlightedSlot (.AsPC%20Gateway (Utilities|Casting|CastToPC_Gateway (Game|GetPlayerController 0))) self)
      ;[1 1 1] hilights the slot
      (Rendering|SetVisibility (Variables|Default|GetHilight) true false)
      ;[1 1 1] tells the player controller to turn on the variable letting everything know a box you are holding is hilighting a slot. then tells a function in the bag to turn on a variable letting it know that it is collding with a box of appropriate size
      (Variables|Default|SetBoxHit OtherActor)
      (Variables|/Game/Core/PC_Gateway.PC_Gateway_C|SetBagOverlapping (.AsPC%20Gateway (Utilities|Casting|CastToPC_Gateway (Game|GetPlayerController 0))) true)
      (Development|PrintString (Utilities|String|EnumtoString (Collision|GetCollisionEnabled (Variables|Default|GetHilight))))
      (Development|PrintString (Utilities|String|EnumtoString (Collision|GetCollisionEnabled (Variables|Default|GetBox)))))))

(event Custom|OnComponentEndOverlap_Event
  (params (OverlappedComponent :type Primitive%20Component%20Object%20Reference) (OtherActor :type Actor%20Object%20Reference) (OtherComp :type Primitive%20Component%20Object%20Reference) (OtherBodyIndex :type Integer))
  (if (== OtherActor (Variables|Default|GetBoxHit))
    (Rendering|SetVisibility (Variables|Default|GetHilight) false false)
    (Variables|Default|SetBoxHit (Variables|Default|GetHitReset))
    (bind _aspc_gateway (Utilities|Casting|CastToPC_Gateway (Game|GetPlayerController 0)))
    (Variables|/Game/Core/PC_Gateway.PC_Gateway_C|SetBagOverlapping _aspc_gateway false)))

(event EventBeginPlay
  (Collision|AssignOnComponentBeginOverlap (Variables|Default|GetSnapBox) (delegate Custom|OnComponentBeginOverlap_Event))
  (Collision|AssignOnComponentEndOverlap (Variables|Default|GetSnapBox) (delegate Custom|OnComponentEndOverlap_Event))
  (Variables|Default|Setbring_In false))

(event Collision|EventActorBeginOverlap
  (params (OtherActor :type Actor%20Object%20Reference)))

(fn ConstructionScript
  (bind _returnvalue (Math|Conversions|ToVector(Float) 2.0))
  (bind _box_size (Variables|Default|GetBox%20size))
  (bind _box (Variables|Default|GetBox))
  (bind _returnvalue_2 (/ _box_size _returnvalue))
  (bind (_x _y _z) (Math|Vector|BreakVector _returnvalue_2))
  (Components|Box|SetBoxExtent _box (Math|Vector|MakeVector (/ _x 2.0) _y (/ _z 2.0)) true)
  (Variables|Default|SetSnapBox _box)
  (Rendering|SetVisibility (Variables|Default|GetHilight) false false))

(fn HideHilight
  (Rendering|SetVisibility (Variables|Default|GetHilight) false false))

(fn RemoveBox)

(fn CollissionOff
  (Collision|SetCollisionEnabled (Variables|Default|GetHilight) "NoCollision"))

(fn Collissionon
  (Collision|SetCollisionEnabled (Variables|Default|GetHilight) "QueryAndPhysics"))