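; BP_BagSlot is a slot actor that marks where a bag of a given size can snap, with highlight and pre-highlight meshes.
; The construction script picks both meshes from BagSizeEnum, assigns their materials, and stores Box as SnapBox, sized to a third of the highlight mesh's half-extents.
; It has no event logic, only functions that toggle each highlight's visibility and the collision of Hilight and Box.
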(fn `Add hilight`
  (`SceneComponent.SetVisibility` (`self.Hilight`) true false))

(fn `CollissionOff`
  (`PrimitiveComponent.SetCollisionEnabled` (`self.Hilight`) "NoCollision")
  (`PrimitiveComponent.SetCollisionEnabled` (`self.Box`) "NoCollision"))

(fn `CollissionOn`
  (`PrimitiveComponent.SetCollisionEnabled` (`self.Hilight`) "QueryAndPhysics")
  (`PrimitiveComponent.SetCollisionEnabled` (`self.Box`) "QueryAndPhysics"))

(fn `Hide Hilight`
  (`SceneComponent.SetVisibility` (`self.Hilight`) false false))

(fn `preHighlight off`
  (`SceneComponent.SetVisibility` (`self.PreHighlight`) false false))

(fn `preHighlight on`
  (`SceneComponent.SetVisibility` (`self.PreHighlight`) true false))

(fn `UserConstructionScript`
  (locals (NewLocalVar :type "Float (double-precision)"))
  (bind _box (`self.Box`))
  (bind (_min _max) (`StaticMeshComponent.GetLocalBounds` (`self.Hilight`)))
  (`SceneComponent.SetVisibility` (`self.Hilight`) (`self.Hilight on`) false)
  (`SceneComponent.SetVisibility` (`self.PreHighlight`) (`self.Hilight on`) false)
  (switch `/Game/Core/Enums/E_BagSizes` (`self.BagSizeEnum`)
    (:`NewEnumerator0`
      (`StaticMeshComponent.SetStaticMesh` (`self.Hilight`) "/Game/ArtAndMeshes/QuasisModule/QasisModuleBags/SM_Bags_SM_BagSmall.SM_Bags_SM_BagSmall")
      (`StaticMeshComponent.SetStaticMesh` (`self.PreHighlight`) "/Game/ArtAndMeshes/QuasisModule/QasisModuleBags/SM_Bags_SM_BagSmall.SM_Bags_SM_BagSmall"))
    (:`NewEnumerator2`
      (`StaticMeshComponent.SetStaticMesh` (`self.Hilight`) "/Game/ArtAndMeshes/QuasisModule/QasisModuleBags/SM_Bags_SM_BagMedium.SM_Bags_SM_BagMedium")
      (`StaticMeshComponent.SetStaticMesh` (`self.PreHighlight`) "/Game/ArtAndMeshes/QuasisModule/QasisModuleBags/SM_Bags_SM_BagMedium.SM_Bags_SM_BagMedium"))
    (:`NewEnumerator3`
      (`StaticMeshComponent.SetStaticMesh` (`self.Hilight`) "/Game/ArtAndMeshes/QuasisModule/QasisModuleBags/SM_Bags_SM_BagLarge.SM_Bags_SM_BagLarge")
      (`StaticMeshComponent.SetStaticMesh` (`self.PreHighlight`) "/Game/ArtAndMeshes/QuasisModule/QasisModuleBags/SM_Bags_SM_BagLarge.SM_Bags_SM_BagLarge"))
    (:`NewEnumerator4`
      (`StaticMeshComponent.SetStaticMesh` (`self.Hilight`) "/Game/ArtAndMeshes/QuasisModule/QasisModuleBags/SM_Bags_SM_BagLargest.SM_Bags_SM_BagLargest")
      (`StaticMeshComponent.SetStaticMesh` (`self.PreHighlight`) "/Game/ArtAndMeshes/QuasisModule/QasisModuleBags/SM_Bags_SM_BagLargest.SM_Bags_SM_BagLargest")))
  (`PrimitiveComponent.SetMaterial` (`self.Hilight`) 0 "/Game/ArtAndMeshes/QuasisModule/QasisModuleBags/Materials/M_LevelTransformMaterial.M_LevelTransformMaterial")
  (`PrimitiveComponent.SetMaterial` (`self.PreHighlight`) 0 "/Game/ArtAndMeshes/QuasisModule/QasisModuleBags/Materials/M_PreHighlight.M_PreHighlight")
  (`BoxComponent.SetBoxExtent` _box (`KismetMathLibrary.MakeVector` (/ (.x (/ (- _max _min) (`KismetMathLibrary.Conv_DoubleToVector` 2.0))) 3.0) (/ (.y (/ (- _max _min) (`KismetMathLibrary.Conv_DoubleToVector` 2.0))) 3.0) (/ (.z (/ (- _max _min) (`KismetMathLibrary.Conv_DoubleToVector` 2.0))) 3.0)) true)
  (set `self.SnapBox` _box))