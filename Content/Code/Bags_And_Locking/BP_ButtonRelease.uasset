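; Button actor that, on any actor overlap, destroys every BP_Bags in the level and, if ButtonPressed is set, plays the Animation of every BP_Door and clears the flag.
; A separate ReleaseModule function, not called within this Blueprint, reveals the door on each BP_FullModelPreset and moves the presets down in Z with sweep.
; The drop distance, SubtractionInt, grows slightly after each preset moved, so successive moves are larger.
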(event `self.ReceiveActorBeginOverlap`
  (params (OtherActor :type "Actor Object Reference"))
  (bind _outactors (`GameplayStatics.GetAllActorsOfClass` "/Game/Code/Bags_And_Locking/Bags/BP_Bags.BP_Bags_C"))
  (for _array_element _outactors
    (`self.K2_DestroyActor` _array_element))
  (if (`self.ButtonPressed`)
    (bind _outactors_2 (`GameplayStatics.GetAllActorsOfClass` "/Game/Code/Bags_And_Locking/BP_Door.BP_Door_C"))
    (for _array_element_2 _outactors_2
      (`/Game/Code/Bags_And_Locking/BP_Door.Animation` _array_element_2)
      (set `self.ButtonPressed` false))))

(event `self.ReceiveTick`
  (params (DeltaSeconds :type "Float (single-precision)")))

(fn `release module`
  (bind _outactors (`GameplayStatics.GetAllActorsOfClass` "/Game/Code/Bags_And_Locking/BP_FullModelPreset.BP_FullModelPreset_C"))
  (for _array_element _outactors
    (`/Game/Code/Bags_And_Locking/BP_FullModelPreset.make door visible` _array_element))
  (bind _outactors_2 (`GameplayStatics.GetAllActorsOfClass` "/Game/Code/Bags_And_Locking/BP_FullModelPreset.BP_FullModelPreset_C"))
  (for _array_element_2 _outactors_2
    (`self.K2_SetActorLocation` _array_element_2 (`KismetMathLibrary.MakeVector` (.x (`self.K2_GetActorLocation` _array_element_2)) (.y (`self.K2_GetActorLocation` _array_element_2)) (- (.z (`self.K2_GetActorLocation` _array_element_2)) (`self.subtraction int`))) true true)
    (set `self.Subtraction int` (+ (`self.Subtraction int`) 0.1))))

(fn `UserConstructionScript`)