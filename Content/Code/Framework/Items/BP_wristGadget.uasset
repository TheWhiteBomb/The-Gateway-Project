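; BP_wristGadget is an unfinished wrist gadget item that picks random tasks for the game.
; On BeginPlay, RNGsetTask rolls two task numbers when Taskworld is true.
; SetTask2, never called here, matches Task2 against TaskArray ranges, recursively rerolling tasks at their call limit, but writes the chosen name to Task1.
; SetTask1, the done checks and the reroll functions are empty stubs.
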(event `self.ReceiveBeginPlay`
  (`self.RNG/set task %`))

(fn `Donecheck1`)

(fn `Donecheck2`)

(fn `Reroll1`)

(fn `Reroll2`)

(fn `RNG/set task %`
  (if (`self.taskworld`)
    (set `self.task1%` (`KismetMathLibrary.RandomIntegerInRange` 1 75))
    (set `self.task2%` (`KismetMathLibrary.RandomIntegerInRange` 1 75))))

(fn `Set Task 2`
  (bind _task2_ (`self.task2%`))
  (for (_array_element _array_index) (`self.TaskArray`)
    (bind (_taskname _minrange _maxrange _timescallable) (break `/Game/Core/S_tasks` _array_element))
    (if (and (>= _task2_ _minrange) (<= _task2_ _maxrange))
      (if (< (`|GetArrayItem` (`self.TimesCalled`) _array_index) _timescallable)
        (set `self.Task1` _taskname)
        (else
          (set `self.task2%` (`KismetMathLibrary.RandomIntegerInRange` 1 75))
          (`self.Set Task 2`))))))

(fn `Set Task1`)

(fn `UserConstructionScript`)