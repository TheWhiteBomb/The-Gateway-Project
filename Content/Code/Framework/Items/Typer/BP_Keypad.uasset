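; BP_Keypad is an interactable keypad actor for typing a code, with minus and decimal keys alongside the digits.
; OnInteract or Initiate enables click events, shows an underscore placeholder matching Temperature's length, and gives each BP_KeypadButtonActor child a reference to the keypad.
; Buttonentered appends ordinary values to the text while CanEnter is true.
; Confirm, back and reset presses have no handling here.
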(event `OnInteract`
  (bind _entercodetext (`self.EnterCodeText`))
  ;[1 1 1] On player interact, assigns base things to an array, and sets up placfeholder text
  (set `PlayerController.bEnableClickEvents` true (`GameplayStatics.GetPlayerController` 0) :!label _label)
  (`TextRenderComponent.K2_SetText` _entercodetext (`KismetSystemLibrary.MakeLiteralText` (`KismetTextLibrary.Conv_StringToText` (`KismetStringLibrary.GetSubstring` "__________" 0 (`KismetStringLibrary.Len` (`self.Temperature`))))))
  (`TextRenderComponent.SetTextRenderColor` _entercodetext (make `Color` 10 10 10 255))
  (bind _output_get (set `self.ButtonArray` (`|MakeArray` (`self.Button_0`) (`self.Button_1`) (`self.Button_2`) (`self.Button_3`) (`self.Button_4`) (`self.Button_5`) (`self.Button_6`) (`self.Button_7`) (`self.Button_8`) (`self.Button_9`) (`self.Button_Minus`) (`self.Button_Decimal`) (`self.Button_Back`) (`self.Button_Reset`) (`self.Button_Check`))))
  (for _array_element _output_get
    (bind _asbp_keypad_button_actor (cast `/Game/Code/Framework/Items/Typer/BP_KeypadButtonActor` (`ChildActorComponent.ChildActor` _array_element)))
    (set `/Game/Code/Framework/Items/Typer/BP_KeypadButtonActor.KeypadActorRef` self _asbp_keypad_button_actor)))

(event `Initiate`
  ;[1 1 1] On player interact, assigns base things to an array, and sets up placfeholder text
  (goto _label))

(event `Button entered`
  (params (value :type Text) (`Confirmed?` :type Boolean) (Back :type Boolean) (Reset :type Boolean))
  (if `Confirmed?`
    _
    (elif Back
      _
      (elif Reset
        _
        (elif (`self.Can Enter`)
          (`TextRenderComponent.K2_SetText` (`self.EnterCodeText`) (`KismetTextLibrary.Conv_StringToText` (`KismetStringLibrary.Concat_StrStr` (`KismetTextLibrary.Conv_TextToString` (`TextRenderComponent.Text` (`self.EnterCodeText`))) (`KismetTextLibrary.Conv_TextToString` value)))))))))

(fn `UserConstructionScript`)