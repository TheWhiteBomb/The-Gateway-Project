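; Wrist gadget whose physical buttons, pressed by the player pawn's finger, drive a tabbed screen for the simulation.
; Overlaps map button components to flat-screen widget buttons, with a shared cooldown and confirmation page; holding reset fills a quit bar on the older screen.
; Init picks two distinct weighted-random tasks from DT_Tasks on first load, and finds the level's day runner, plus the box delivery manager in the Loading level.
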(event `self.ReceiveTick`
  (params (DeltaSeconds :type "Float (single-precision)"))
  (set `self.TextCooldown` (+ DeltaSeconds (`self.TextCooldown`)))
  (set `self.GameCount` (+ DeltaSeconds (`self.GameCount`)))
  (set `self.LevelCount` (+ DeltaSeconds (`self.LevelCount`)))
  (set `self.ButtonCooldown` (- (`self.ButtonCooldown`) DeltaSeconds))
  (`|ExecutionSequence`
    (:`then_0`
      (if (`self.HoldingReset`)
        (set `self.QuitCounter` (+ (/ DeltaSeconds 5.0) (`self.QuitCounter`)))))
    (:`then_1`
      (`/Game/Code/wristGadget/WristScreen/BP_WristScreen.SetQuitBarProgress` (cast `/Game/Code/wristGadget/WristScreen/BP_WristScreen` (`WidgetComponent.GetWidget` (`self.ScreenOLD`)) :!pure true) (and (`self.HoldingReset`) (< (`self.QuitCounter`) 1.0)) (`KismetMathLibrary.FClamp` (`self.QuitCounter`)))
      (if (>= (`self.QuitCounter`) 1.0)
        (set `self.HoldingReset` false)
        (`/Game/Code/wristGadget/WristScreen/BP_WristScreen.LoadConfirmation` (`self.Widget`) "NewEnumerator3" "Are you sure you'd like to quit the simulation?")))))

(event `self.ReceiveBeginPlay`
  (set `self.ButtonList` (`|MakeArray` (`self.ResetButton`) (`self.LevelButton`) (`self.NextButton`)))
  (set `self.FlatScreen` (cast `/Game/Code/WristUI/WBP_FlatScreen` (`WidgetComponent.GetWidget` (`self.WristUI`)) :!pure true))
  (set `self.RealActorButtonTable` (`|MakeMap` (`self.TabControlButton`) (`/Game/Code/WristUI/WBP_FlatScreen.ControlTabButton` (`self.FlatScreen`)) (`self.TabPhaseButton`) (`/Game/Code/WristUI/WBP_FlatScreen.PhaseTabButton` (`self.FlatScreen`)) (`self.TabDataButton`) (`/Game/Code/WristUI/WBP_FlatScreen.InfoTabButton` (`self.FlatScreen`)) (`self.TabTaskButton`) (`/Game/Code/WristUI/WBP_FlatScreen.TaskTabButton` (`self.FlatScreen`)) :!type "ActorComponent Object Reference"))
  (set `self.RealActorIndexTable` (`|MakeArray` (`self.OptionButton0`) (`self.OptionButton1`) (`self.OptionButton2`) (`self.OptionButton3`) :!type "ActorComponent Object Reference")))

(event `Init`
  (bind _text_handler (`self.Text Handler`))
  (bind _returnvalue (`KismetStringLibrary.Conv_NameToString` (`/Game/Code/ProjectLibraries/BPML_Global.GetLevelName`)))
  (set `self.LevelCount` 0.0)
  (`/Game/Code/ProjectLibraries/BPML_Actor.SingleLoadEventLock`
    (:`First Load Ever`
      (bind _outrownames (`DataTableFunctionLibrary.GetDataTableRowNames` "/Game/Data/DT_Tasks.DT_Tasks"))
      (for _array_element _outrownames
        (bind _returnvalue_2 (`|GetDataTableRow` "/Game/Data/DT_Tasks.DT_Tasks" _array_element)
          (:`then`
            (`KismetArrayLibrary.Array_Add` (`self.TaskArray`) _returnvalue_2))))
      ;[0 1 0.2593 0.5] Randomize Tasks
      (`self.SetTasks`)
      (set `/Game/Code/wristGadget/RenderTargets/BP_text.Tasks Used` (`self.Task Selected`) (`self.Text Handler`))
      ;[0 0.8628 1 0.5] Initialize Widget
      (bind _returnvalue_3 (`|CreateWidget` "/Game/Code/wristGadget/WristScreen/BP_WristScreen.BP_WristScreen_C" (`GameplayStatics.GetPlayerController` 0)))
      (`WidgetComponent.SetWidget` (`self.ScreenOLD`) _returnvalue_3)
      (set `self.Widget` _returnvalue_3)
      (`KismetSystemLibrary.PrintString` (`KismetStringLibrary.Concat_StrStr` "Loading Level: \"" _returnvalue "\"") true true (struct :`R` 1.0 :`B` 0.85601 :`A` 1.0))
      (`|ExecutionSequence`
        (:`then_0`
          (switch `string` _returnvalue :!label _label
            (:`Default`
              ;[0 0.304 1 0.5] Initialize Day Runner Reference
              ;;[0 1 0.8645 0.5] Default
              (bind _outactors (`GameplayStatics.GetAllActorsOfClass` "/Script/The_Gateway_Project.DayCycleRunner"))
              (bind _output (`|GetArrayItem` _outactors))
              (`/Engine/EditorBlueprintResources/StandardMacros.IsValid` _output
                (:`Is Valid`
                  (set `self.DayRunner` _output))))
            (:`Loading`
              ;;[0 0.4252 1 0.5] Loading Level
              (bind _outactors_2 (`GameplayStatics.GetAllActorsOfClass` "/Script/The_Gateway_Project.BoxDeliveryDayRunner"))
              (set `self.DayRunner` (`|GetArrayItem` _outactors_2))
              (bind _outactors_3 (`GameplayStatics.GetAllActorsOfClass` "/Script/The_Gateway_Project.BoxDeliveryManager"))
              (set `self.Box Delivery Manager` (`|GetArrayItem` _outactors_3)))))
        (:`then_1`
          (`KismetSystemLibrary.DelayUntilNextTick`)
          (`/Game/Code/wristGadget/RenderTargets/BP_text.event set everything` _text_handler)
          (`/Game/Code/wristGadget/RenderTargets/BP_text.Update Screen` _text_handler)
          (`self.InitBoxes`))))
    (:`First Load Into Level`
      (goto _label))))

(event `self.OptionButton0.OnComponentBeginOverlap`
  (params (OverlappedComponent :type "PrimitiveComponent Object Reference") (OtherActor :type "Actor Object Reference") (OtherComp :type "PrimitiveComponent Object Reference") (OtherBodyIndex :type Integer) (bFromSweep :type Boolean) (SweepResult :type "HitResult Structure (by ref)"))
  (`self.ButtonComponentActivate` OverlappedComponent OtherComp))

(event `self.ConfirmYesButton.OnComponentBeginOverlap`
  (params (OverlappedComponent :type "PrimitiveComponent Object Reference") (OtherActor :type "Actor Object Reference") (OtherComp :type "PrimitiveComponent Object Reference") (OtherBodyIndex :type Integer) (bFromSweep :type Boolean) (SweepResult :type "HitResult Structure (by ref)"))
  (`self.ButtonComponentActivate` OverlappedComponent OtherComp))

(event `self.TabControlButton.OnComponentBeginOverlap`
  (params (OverlappedComponent :type "PrimitiveComponent Object Reference") (OtherActor :type "Actor Object Reference") (OtherComp :type "PrimitiveComponent Object Reference") (OtherBodyIndex :type Integer) (bFromSweep :type Boolean) (SweepResult :type "HitResult Structure (by ref)"))
  (`self.ButtonComponentActivate` OverlappedComponent OtherComp))

(event `self.TabCloseButton.OnComponentBeginOverlap`
  (params (OverlappedComponent :type "PrimitiveComponent Object Reference") (OtherActor :type "Actor Object Reference") (OtherComp :type "PrimitiveComponent Object Reference") (OtherBodyIndex :type Integer) (bFromSweep :type Boolean) (SweepResult :type "HitResult Structure (by ref)"))
  (`self.IsFIngerComponent` OtherComp
    (:`true`
      (set `/Game/Code/ZeroGravity/BP_SharedPawn.Wrist UI Active` false (cast `/Game/Code/ZeroGravity/BP_SharedPawn` (`GameplayStatics.GetPlayerPawn` 0) :!pure true)))))

(event `self.OptionButton1.OnComponentBeginOverlap`
  (params (OverlappedComponent :type "PrimitiveComponent Object Reference") (OtherActor :type "Actor Object Reference") (OtherComp :type "PrimitiveComponent Object Reference") (OtherBodyIndex :type Integer) (bFromSweep :type Boolean) (SweepResult :type "HitResult Structure (by ref)"))
  (`self.ButtonComponentActivate` OverlappedComponent OtherComp))

(event `self.ConfirmNoButton.OnComponentBeginOverlap`
  (params (OverlappedComponent :type "PrimitiveComponent Object Reference") (OtherActor :type "Actor Object Reference") (OtherComp :type "PrimitiveComponent Object Reference") (OtherBodyIndex :type Integer) (bFromSweep :type Boolean) (SweepResult :type "HitResult Structure (by ref)"))
  (`self.ButtonComponentActivate` OverlappedComponent OtherComp))

(event `self.TabPhaseButton.OnComponentBeginOverlap`
  (params (OverlappedComponent :type "PrimitiveComponent Object Reference") (OtherActor :type "Actor Object Reference") (OtherComp :type "PrimitiveComponent Object Reference") (OtherBodyIndex :type Integer) (bFromSweep :type Boolean) (SweepResult :type "HitResult Structure (by ref)"))
  (`self.ButtonComponentActivate` OverlappedComponent OtherComp))

(event `self.OptionButton2.OnComponentBeginOverlap`
  (params (OverlappedComponent :type "PrimitiveComponent Object Reference") (OtherActor :type "Actor Object Reference") (OtherComp :type "PrimitiveComponent Object Reference") (OtherBodyIndex :type Integer) (bFromSweep :type Boolean) (SweepResult :type "HitResult Structure (by ref)"))
  (`self.ButtonComponentActivate` OverlappedComponent OtherComp))

(event `self.TabDataButton.OnComponentBeginOverlap`
  (params (OverlappedComponent :type "PrimitiveComponent Object Reference") (OtherActor :type "Actor Object Reference") (OtherComp :type "PrimitiveComponent Object Reference") (OtherBodyIndex :type Integer) (bFromSweep :type Boolean) (SweepResult :type "HitResult Structure (by ref)"))
  (`self.ButtonComponentActivate` OverlappedComponent OtherComp))

(event `self.OptionButton3.OnComponentBeginOverlap`
  (params (OverlappedComponent :type "PrimitiveComponent Object Reference") (OtherActor :type "Actor Object Reference") (OtherComp :type "PrimitiveComponent Object Reference") (OtherBodyIndex :type Integer) (bFromSweep :type Boolean) (SweepResult :type "HitResult Structure (by ref)"))
  (`self.ButtonComponentActivate` OverlappedComponent OtherComp))

(event `self.TabTaskButton.OnComponentBeginOverlap`
  (params (OverlappedComponent :type "PrimitiveComponent Object Reference") (OtherActor :type "Actor Object Reference") (OtherComp :type "PrimitiveComponent Object Reference") (OtherBodyIndex :type Integer) (bFromSweep :type Boolean) (SweepResult :type "HitResult Structure (by ref)"))
  (`self.ButtonComponentActivate` OverlappedComponent OtherComp))

(event `self.OptionButton0.OnComponentEndOverlap`
  (params (OverlappedComponent :type "PrimitiveComponent Object Reference") (OtherActor :type "Actor Object Reference") (OtherComp :type "PrimitiveComponent Object Reference") (OtherBodyIndex :type Integer))
  (`self.ReleaseButtonFromComponent` OverlappedComponent OtherComp))

(event `self.TabControlButton.OnComponentEndOverlap`
  (params (OverlappedComponent :type "PrimitiveComponent Object Reference") (OtherActor :type "Actor Object Reference") (OtherComp :type "PrimitiveComponent Object Reference") (OtherBodyIndex :type Integer))
  (`self.ReleaseButtonFromComponent` OverlappedComponent OtherComp))

(event `self.OptionButton1.OnComponentEndOverlap`
  (params (OverlappedComponent :type "PrimitiveComponent Object Reference") (OtherActor :type "Actor Object Reference") (OtherComp :type "PrimitiveComponent Object Reference") (OtherBodyIndex :type Integer))
  (`self.ReleaseButtonFromComponent` OverlappedComponent OtherComp))

(event `self.TabTaskButton.OnComponentEndOverlap`
  (params (OverlappedComponent :type "PrimitiveComponent Object Reference") (OtherActor :type "Actor Object Reference") (OtherComp :type "PrimitiveComponent Object Reference") (OtherBodyIndex :type Integer))
  (`self.ReleaseButtonFromComponent` OverlappedComponent OtherComp))

(event `self.OptionButton2.OnComponentEndOverlap`
  (params (OverlappedComponent :type "PrimitiveComponent Object Reference") (OtherActor :type "Actor Object Reference") (OtherComp :type "PrimitiveComponent Object Reference") (OtherBodyIndex :type Integer))
  (`self.ReleaseButtonFromComponent` OverlappedComponent OtherComp))

(event `self.TabPhaseButton.OnComponentEndOverlap`
  (params (OverlappedComponent :type "PrimitiveComponent Object Reference") (OtherActor :type "Actor Object Reference") (OtherComp :type "PrimitiveComponent Object Reference") (OtherBodyIndex :type Integer))
  (`self.ReleaseButtonFromComponent` OverlappedComponent OtherComp))

(event `self.OptionButton3.OnComponentEndOverlap`
  (params (OverlappedComponent :type "PrimitiveComponent Object Reference") (OtherActor :type "Actor Object Reference") (OtherComp :type "PrimitiveComponent Object Reference") (OtherBodyIndex :type Integer))
  (`self.ReleaseButtonFromComponent` OverlappedComponent OtherComp))

(event `self.TabDataButton.OnComponentEndOverlap`
  (params (OverlappedComponent :type "PrimitiveComponent Object Reference") (OtherActor :type "Actor Object Reference") (OtherComp :type "PrimitiveComponent Object Reference") (OtherBodyIndex :type Integer))
  (`self.ReleaseButtonFromComponent` OverlappedComponent OtherComp))

(fn `ButtonComponentSetPressed`
  (params (Component :type "Object Object Reference") (Enabled :type Boolean))
  (bind _flatscreen (`self.FlatScreen`))
  (bind _flatscreen_2 (`self.FlatScreen`))
  (`/Engine/EditorBlueprintResources/StandardMacros.IsValid` Component
    (:`Is Valid`
      (if (not Enabled)
        (set `self.ReleasedButton` true))
      (bind (_tabbutton _displaybutton _istabbutton _isconfirmation _confirmed) (`self.GetButtonForComponent` Component))
      (if _istabbutton
        ; Switch tabs
        (`/Game/Code/WristUI/WBP_TabButton.SetPressed` _tabbutton Enabled)
        ; Converges every endpoint to reset the button cooldown. This happens here to prevent overlapping.
        (set `self.ButtonCooldown` (`self.ButtonCooldownMax`) :!label _label)
        (elif _isconfirmation
          ;[0.15 0.15 0.15 0.4783] Finally activate functionality for whatever button we have confirmed
          (if (== (`WidgetSwitcher.ActiveWidgetIndex` (`/Game/Code/WristUI/WBP_FlatScreen.TabMenu` (`self.FlatScreen`))) 4)
            (`/Game/Code/WristUI/WBP_DisplayButton.Confirm` _displaybutton _confirmed)
            (`WidgetSwitcher.SetActiveWidgetIndex` (`/Game/Code/WristUI/WBP_FlatScreen.TabMenu` _flatscreen) (`/Game/Code/WristUI/WBP_FlatScreen.TabBeforeConfirmation` _flatscreen))
            ; Hides the confirmation popup if necessary
            (`/Game/Code/WristUI/WBP_FlatScreen.CheckConfirmationVisible` _flatscreen_2 :!label _label_2)
            (goto _label))
          (elif (and (`KismetSystemLibrary.IsValid` _displaybutton) (!= (`WidgetSwitcher.ActiveWidgetIndex` (`/Game/Code/WristUI/WBP_FlatScreen.TabMenu` (`self.FlatScreen`))) 4))
            (if (`/Game/Code/WristUI/WBP_DisplayButton.RequiresConfirmation` _displaybutton)
              ; Delay functionality for confirmation buttons
              (if Enabled
                (`/Game/Code/WristUI/WBP_FlatScreen.SetConfirmation` _flatscreen_2 _displaybutton)
                (`WidgetSwitcher.SetActiveWidgetIndex` (`/Game/Code/WristUI/WBP_FlatScreen.TabMenu` _flatscreen_2) 4)
                (goto _label_2))
              (else
                ; Activate functionality for regular buttons
                (if (`/Game/Code/WristUI/WBP_DisplayButton.CanBePressed` _displaybutton)
                  (`/Game/Code/WristUI/WBP_DisplayButton.SetPressed` _displaybutton Enabled)
                  (goto _label))))))))))

(fn `GetButtonForComponent`
  (params (Component :type "Object Object Reference"))
  (returns (TabButton :type "/Game/Code/WristUI/WBP_TabButton Object Reference") (DisplayButton :type "/Game/Code/WristUI/WBP_DisplayButton Object Reference") (IsTabButton :type Boolean) (IsConfirmation :type Boolean) (Confirmed :type Boolean))
  (bind _confirmationbutton (`/Game/Code/WristUI/WBP_FlatScreen.ConfirmationButton` (`self.FlatScreen`)))
  (`/Engine/EditorBlueprintResources/StandardMacros.IsValid` Component
    (:`Is Valid`
      (bind _keys (`BlueprintMapLibrary.Map_Keys` (`self.RealActorButtonTable`)))
      (for _array_element _keys
        (if (== _array_element Component)
          (return (`BlueprintMapLibrary.Map_Find` (`self.RealActorButtonTable`) _array_element) null true false false)))
      (if (== Component (`self.ConfirmYesButton`))
        (return null _confirmationbutton false true true)
        (elif (== Component (`self.ConfirmNoButton`))
          (return null _confirmationbutton false true false)
          (else
            (for (_array_element_2 _array_index) (`self.RealActorIndexTable`)
              (if (== _array_element_2 Component)
                (bind _buttons (`self.GetButtonsFromTab` (`WidgetSwitcher.GetActiveWidget` (`/Game/Code/WristUI/WBP_FlatScreen.TabMenu` (`self.FlatScreen`)))))
                (return null (`|GetArrayItem` _buttons _array_index) false false false)))
            (`KismetSystemLibrary.PrintString` (`KismetStringLibrary.Concat_StrStr` "COULD NOT FIND BUTTON FOR COMPONENT \"" (`KismetSystemLibrary.GetDisplayName` Component) "\"!"))))))
    (:`Is Not Valid`
      (`KismetSystemLibrary.PrintString` "INVALID COMPONENT" true true (struct :`R` 1.0 :`G` 0.08761 :`A` 1.0) 999999.0))))

(fn `GetButtonsFromTab`
  (params (Widget :type "Widget Object Reference"))
  (returns (Buttons :type "Array of /Game/Code/WristUI/WBP_DisplayButton Object Reference"))
  (bind _aswbp_control_tab (cast `/Game/Code/WristUI/Tabs/WBP_ControlTab` Widget)
    (:`then`
      (return (`/Game/Code/WristUI/Tabs/WBP_ControlTab.Buttons` _aswbp_control_tab)))
    (:`CastFailed`
      (bind _aswbp_phase_tab (cast `/Game/Code/WristUI/Tabs/WBP_PhaseTab` Widget)
        (:`then`
          (return (`/Game/Code/WristUI/Tabs/WBP_PhaseTab.Buttons` _aswbp_phase_tab)))
        (:`CastFailed`
          (bind _aswbp_data_tab (cast `/Game/Code/WristUI/Tabs/WBP_DataTab` Widget)
            (:`then`
              (return (`/Game/Code/WristUI/Tabs/WBP_DataTab.Buttons` _aswbp_data_tab)))
            (:`CastFailed`
              (bind _aswbp_task_tab (cast `/Game/Code/WristUI/Tabs/WBP_TaskTab` Widget)
                (:`then`
                  (return (`/Game/Code/WristUI/Tabs/WBP_TaskTab.Buttons` _aswbp_task_tab)))
                (:`CastFailed`
                  (return (`|MakeArray`)))))))))))

(fn `GetRandomTask`
  (params (RestartIfFound :type Name :default "None") (TaskNumber :type Integer))
  (returns (Found :type "/Game/Core/Structures/S_TaskSelected Structure"))
  (locals (EncounterCounter :type "Float (double-precision)") (InRange :type Boolean) (SetRandom :type "Float (double-precision)"))
  (bind _encountercounter (`local.EncounterCounter`))
  (set `local.SetRandom` (`KismetMathLibrary.RandomFloat`))
  (for _array_element (`self.TaskArray`)
    (bind (_taskname _selectionchance _timescallable _tasktype _taskrequired _taskrequiredextension _hasextension) (break `/Game/Core/Structures/S_tasks` _array_element))
    (bind _returnvalue (+ _encountercounter (`KismetMathLibrary.Abs` _selectionchance)))
    (set `local.InRange` (`KismetMathLibrary.InRange_FloatFloat` (`local.SetRandom`) _encountercounter _returnvalue))
    (set `local.EncounterCounter` _returnvalue)
    (if (`local.InRange`)
      (if (== RestartIfFound _taskname)
        (bind _found (`self.GetRandomTask` RestartIfFound TaskNumber))
        (return _found)
        (else
          (return (make `/Game/Core/Structures/S_TaskSelected` TaskNumber _taskname _tasktype _taskrequired _taskrequiredextension _hasextension)))))))

(fn `InitBoxes`
  (bind _outactors (`GameplayStatics.GetAllActorsOfClass` "/Game/Code/Bags_And_Locking/Locking/BP_BagSlot.BP_BagSlot_C"))
  (set `self.Boxes` _outactors))

(fn `NextDay`
  (bind _dayrunner (`self.DayRunner`))
  (bind _box_delivery_manager (`self.Box Delivery Manager`))
  (if (and (`KismetSystemLibrary.IsValid` _box_delivery_manager) (not (`DayCycleRunner.IsTransitioning` _dayrunner)) (< (`DayCycleRunner.GetDayCount` _dayrunner) (`BoxDeliveryManager.TotalDays` _box_delivery_manager)))
    (`DayCycleRunner.ProgressDaySequence` _dayrunner 0)))

(fn `Set Task1`)

(fn `SetTasks`
  (locals (SelectionMaxChance :type "Float (double-precision)"))
  (bind _selectionmaxchance (`local.SelectionMaxChance`))
  (bind _task_selected (`self.Task Selected`))
  ;[0.125 1 0.8296 0.5] Count Chances
  (for _array_element (`self.TaskArray`)
    (set `local.SelectionMaxChance` (+ (`KismetMathLibrary.Abs` (`.SelectionChance_49_415AAC5CB3441E82059BE5BCADE12AA6` (break `/Game/Core/Structures/S_tasks` _array_element))) (`local.SelectionMaxChance`))))
  (if (`KismetMathLibrary.InRange_FloatFloat` _selectionmaxchance 0.99 1.01)
    ;[0.1427 0.3969 1 0.5] Randomize Tasks
    (bind _found (`self.GetRandomTask` "None" 2))
    (`KismetArrayLibrary.Array_Set` _task_selected 1 _found)
    (bind _found_2 (`self.GetRandomTask` (`.TaskName_6_E1D2614A80418031F464488B1C001021` (break `/Game/Core/Structures/S_TaskSelected` _found)) 3))
    (`KismetArrayLibrary.Array_Set` _task_selected 2 _found_2)
    (for _array_element_2 _task_selected
      _)
    (else
      ;[1 1 0.2083 0.5] Fail When Chances Don't Add Up To 1
      (`KismetSystemLibrary.PrintString` "TASK SELECTION CONFIG DOES NOT ADD UP TO 1!" true true (struct :`R` 0.745404 :`G` 0.099899 :`B` 0.084376 :`A` 1.0) 99999.0)
      (`KismetSystemLibrary.PrintString` (`KismetStringLibrary.Concat_StrStr` "Total Task Selection Chance: " (`KismetStringLibrary.Conv_DoubleToString` _selectionmaxchance)) true true (struct :`R` 0.745404 :`G` 0.099899 :`B` 0.084376 :`A` 1.0) 99999.0))))

(fn `UpdateBoxes`
  (locals (FoundBoxes :type Integer))
  (if (`/Game/Code/ProjectLibraries/BPML_Global.IsLevel` "Loading")
    (for _array_element (`self.Boxes`)
      (if (`/Game/Code/Bags_And_Locking/Locking/BP_BagSlot.In Use` _array_element)
        (set `local.FoundBoxes` (+ (`local.FoundBoxes`) 1))))
    (set `/Game/Code/Persistent/GatewayGameInstance._BoxesInUse` (`local.FoundBoxes`) (`/Game/Code/ProjectLibraries/BPML_Global.GetGatewayGameInstance`))))

(fn `UserConstructionScript`
  (set `self.ButtonList` (`|MakeArray` (`self.ResetButton`) (`self.NextButton`) (`self.LevelButton`))))