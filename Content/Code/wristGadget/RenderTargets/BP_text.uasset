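; BP_text is the task data handler behind the wrist gadget's task display.
; On BeginPlay it loads DT_TaskDisplays into a struct array and registers itself with the level's BP_wristGadget.
; It increments the three active tasks by overlapped box type, including optional extension counters, and flags completed ones.
; A separately counted trash task resets the array and tasks when complete, while screen functions cycle three displays through the gadget's widget.
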(event `self.ReceiveTick`
  (params (DeltaSeconds :type "Float (single-precision)")))

(event `event set everything`
  ; Sets the tasks as array indexes for the text structure, when i need to switch screens. i pull that index and apply it to the structure
  (for (_array_element _array_index) (`self.Tasks Used`)
    (for (_array_element_2 _array_index_2) (`self.Text`)
      (if (== (`.TaskName_32_95B8899A514693F43E4469B931192DB9` (break `/Game/Core/S_Print` _array_element_2)) (`.TaskName_6_E1D2614A80418031F464488B1C001021` (break `/Game/Core/S_TaskSelected` _array_element)))
        (if (== _array_index 0)
          (set `self.task 1` _array_index_2)
          (break)
          (elif (== _array_index 1)
            (set `self.Task2` _array_index_2)
            (break)
            (else
              (set `self.Task 3` _array_index_2)
              (break))))))))

(event `self.ReceiveBeginPlay`
  (bind _outrownames (`DataTableFunctionLibrary.GetDataTableRowNames` "/Game/Data/DT_TaskDisplays.DT_TaskDisplays"))
  (for _array_element _outrownames
    (bind _returnvalue (`|GetDataTableRow` "/Game/Data/DT_TaskDisplays.DT_TaskDisplays" _array_element)
      (:`then`
        (`KismetArrayLibrary.Array_Add` (`self.Text`) _returnvalue))))
  (`self.InitializeWristGadgetLocation`))

(fn `Add To Trash`
  (bind (_taskname _taskprogress _taskrequired _taskprogressextension _taskrequiredextension _hasextension _boxtype _boxtypeextension) (break `/Game/Core/S_Print` (`|GetArrayItem` (`self.Text`) 10)))
  (bind _returnvalue (+ _taskprogress 1))
  (if (`|EnumEquality` (`self.overlapped box`) "NewEnumerator13")
    (if (== _returnvalue _taskrequired)
      (set `self.Text` (`self.Text Reset`))
      (set `self.Trash Task` false)
      (bind _outactors (`GameplayStatics.GetAllActorsOfClass` "/Game/Code/wristGadget/BP_wristGadget.BP_wristGadget_C"))
      (for _array_element _outactors
        (`/Game/Code/wristGadget/BP_wristGadget.Set Task1` _array_element)
        (`/Game/Code/wristGadget/BP_wristGadget.SetTasks` _array_element)
        (`self.Update Screen` :!label _label))
      (else
        (`KismetArrayLibrary.Array_Set` (`self.Text`) 10 (make `/Game/Core/S_Print` _taskname _returnvalue _taskrequired _taskprogressextension _taskrequiredextension _hasextension _boxtype _boxtypeextension))
        (goto _label)))))

(fn `InitializeWristGadgetLocation`
  (bind _outactors (`GameplayStatics.GetAllActorsOfClass` "/Game/Code/wristGadget/BP_wristGadget.BP_wristGadget_C"))
  (bind _output (`|GetArrayItem` _outactors))
  (`/Engine/EditorBlueprintResources/StandardMacros.IsValid` _output
    (:`Is Valid`
      (bind _output_get (set `self.WristGadget` _output))
      (set `/Game/Code/wristGadget/BP_wristGadget.Text Handler` self _output_get)
      (`/Game/Code/wristGadget/BP_wristGadget.Init` _output_get))
    (:`Is Not Valid`
      (`KismetSystemLibrary.PrintString` "BP_WRISTGADGET DOES NOT EXIST IN CURRENT LEVEL BUT BP_TEXT DOES!" true true (struct :`R` 1.0 :`G` 0.034973 :`A` 1.0) 9999.0))))

(fn `Subtract from trash`
  (bind (_taskname _taskprogress _taskrequired _taskprogressextension _taskrequiredextension _hasextension _boxtype _boxtypeextension) (break `/Game/Core/S_Print` (`|GetArrayItem` (`self.Text`) 10)))
  (bind _returnvalue (+ _taskprogress -1))
  (if (`|EnumEquality` (`self.overlapped box`) "NewEnumerator13")
    (if (== _returnvalue _taskrequired)
      (set `self.Text` (`self.Text Reset`))
      (set `self.Trash Task` false)
      (bind _outactors (`GameplayStatics.GetAllActorsOfClass` "/Game/Code/wristGadget/BP_wristGadget.BP_wristGadget_C"))
      (for _array_element _outactors
        (`/Game/Code/wristGadget/BP_wristGadget.Set Task1` _array_element)
        (`/Game/Code/wristGadget/BP_wristGadget.SetTasks` _array_element))
      (else
        (`KismetArrayLibrary.Array_Set` (`self.Text`) 10 (make `/Game/Core/S_Print` _taskname _returnvalue _taskrequired _taskprogressextension _taskrequiredextension _hasextension _boxtype _boxtypeextension))))))

(fn `Switch Screen`
  (if (== (`self.displayed screen`) 2)
    (set `self.displayed screen` 0)
    (else
      (set `self.displayed screen` (+ (`self.displayed screen`) 1))))
  (`self.Update Screen`))

(fn `Update Screen`
  (bind _displayed_screen (`self.displayed screen`))
  (`KismetSystemLibrary.PrintString` (`KismetStringLibrary.Conv_IntToString` _displayed_screen) true true (struct :`R` 1.0 :`G` 0.07344 :`B` 0.632782 :`A` 1.0))
  (`/Game/Code/wristGadget/WristScreen/BP_WristScreen.LoadScreen` (`/Game/Code/wristGadget/BP_wristGadget.Widget` (`self.WristGadget`)) (`|GetArrayItem` (`self.Text`) (`.TaskNumber_3_C3443A6E5246B964E5AC1096B74E2172` (break `/Game/Core/S_TaskSelected` (`|GetArrayItem` (`/Game/Code/wristGadget/BP_wristGadget.Task Selected` (`self.WristGadget`)) _displayed_screen)))) _displayed_screen))

(fn `Update Variables`
  (bind (_taskname _taskprogress _taskrequired _taskprogressextension _taskrequiredextension _hasextension) (break `/Game/Core/S_Print` (`|GetArrayItem` (`self.Text`) (`self.Task 3`))))
  (bind (_taskname_2 _taskprogress_2 _taskrequired_2 _taskprogressextension_2 _taskrequiredextension_2 _hasextension_2) (break `/Game/Core/S_Print` (`|GetArrayItem` (`self.Text`) (`self.task 1`))))
  (bind (_taskname_3 _taskprogress_3 _taskrequired_3 _taskprogressextension_3 _taskrequiredextension_3 _hasextension_3) (break `/Game/Core/S_Print` (`|GetArrayItem` (`self.Text`) (`self.Task2`))))
  (bind _returnvalue (== _taskprogress _taskrequired))
  (bind _returnvalue_2 (== _taskprogress_2 _taskrequired_2))
  (bind _returnvalue_3 (== _taskprogress_3 _taskrequired_3))
  (if (not (`self.Trash Task`))
    (for (_array_element _array_index) (`self.Text`)
      (if (or (== _array_index (`self.task 1`)) (== _array_index (`self.Task2`)) (== _array_index (`self.Task 3`)))
        (bind (_taskname_4 _taskprogress_4 _taskrequired_4 _taskprogressextension_4 _taskrequiredextension_4 _hasextension_4 _boxtype _boxtypeextension) (break `/Game/Core/S_Print` _array_element))
        (if _hasextension_4
          (bind _returnvalue_4 (`|EnumEquality` _boxtype (`self.overlapped box`)))
          (if _returnvalue_4
            (bind _returnvalue_5 (== _taskprogress_4 _taskrequired_4))
            (if (not _returnvalue_5)
              (`KismetArrayLibrary.Array_Set` (`self.Text`) (`self.Array Set Index`) (make `/Game/Core/S_Print` _taskname_4 (+ _taskprogress_4 1) _taskrequired_4 _taskprogressextension_4 _taskrequiredextension_4 _hasextension_4 _boxtype _boxtypeextension) :!label _label)
              (`|ExecutionSequence` :!label _label_2
                (:`then_0`
                  (if _hasextension_2
                    (if (and _returnvalue_2 (== _taskprogressextension_2 _taskrequiredextension_2))
                      (`KismetArrayLibrary.Array_Set` (`self.tasks Done`) 0 true :!label _label_3))
                    (elif _returnvalue_2
                      (goto _label_3))))
                (:`then_1`
                  (if _hasextension_3
                    (if (and _returnvalue_3 (== _taskprogressextension_3 _taskrequiredextension_3))
                      (`KismetArrayLibrary.Array_Set` (`self.tasks Done`) 1 true :!label _label_4))
                    (elif _returnvalue_3
                      (goto _label_4))))
                (:`then_2`
                  (if _hasextension
                    (if (and _returnvalue (== _taskprogressextension _taskrequiredextension))
                      (`KismetArrayLibrary.Array_Set` (`self.tasks Done`) 2 true :!label _label_5))
                    (elif _returnvalue
                      (goto _label_5))))
                (:`then_3`
                  (for (_array_element_2 _array_index_2) (`self.tasks Done`)
                    (if _array_element_2
                      (if (== _array_index_2 (`self.Task Amount Index`))
                        (set `self.Trash Task` false))
                      (else
                        (break)))))))
            (elif (`|EnumEquality` _boxtypeextension (`self.overlapped box`))
              (if (not (== _taskprogressextension_4 _taskrequiredextension_4))
                (`KismetArrayLibrary.Array_Set` (`self.Text`) (`self.Array Set Index`) (make `/Game/Core/S_Print` _taskname_4 _taskprogress_4 _taskrequired_4 (+ _taskprogressextension_4 1) _taskrequiredextension_4 _hasextension_4 _boxtype _boxtypeextension))
                (goto _label_2))))
          (elif _returnvalue_4
            (if (not _returnvalue_5)
              (goto _label))))))))

(fn `UserConstructionScript`)