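; BP_TaskUpdate is a trigger volume that advances task progress when a BP_Bags actor overlaps its box.
; On BeginPlay it caches the first BP_text actor as TextManager, which holds the task list.
; On overlap it credits the first unfinished task segment, main or optional extension, matching the bag's type.
; It then calls UpdateVariables on TextManager.
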(event `self.ReceiveBeginPlay`
  (bind _outactors (`GameplayStatics.GetAllActorsOfClass` "/Game/Code/wristGadget/RenderTargets/BP_text.BP_text_C"))
  (bind _output (`|GetArrayItem` _outactors))
  (`/Engine/EditorBlueprintResources/StandardMacros.IsValid` _output
    (:`Is Valid`
      (set `self.TextManager` _output))
    (:`Is Not Valid`
      (`KismetSystemLibrary.PrintString` "BP_TEXT NOT FOUND BY TASK UPDATER" true true (struct :`R` 1.0 :`G` 0.025733 :`A` 1.0) 99999999.0))))

(event `self.Box.OnComponentBeginOverlap`
  (params (OverlappedComponent :type "PrimitiveComponent Object Reference") (OtherActor :type "Actor Object Reference") (OtherComp :type "PrimitiveComponent Object Reference") (OtherBodyIndex :type Integer) (bFromSweep :type Boolean) (SweepResult :type "HitResult Structure (by ref)"))
  (bind _type (`/Game/Code/Bags_And_Locking/Bags/BP_Bags.Type` (cast `/Game/Code/Bags_And_Locking/Bags/BP_Bags` OtherActor :!pure true)))
  (bind _text (`/Game/Code/wristGadget/RenderTargets/BP_text.Text` (`self.TextManager`)))
  (`|ExecutionSequence`
    (:`then_0`
      (for (_array_element _array_index) _text
        (bind (_taskname _taskprogress _taskrequired _taskprogressextension _taskrequiredextension _hasextension _boxtype _boxtypeextension) (break `/Game/Core/S_Print` _array_element))
        (if (and (< _taskprogress _taskrequired) (`|EnumEquality` _boxtype _type))
          (`KismetArrayLibrary.Array_Set` _text _array_index (`/Game/Code/ProjectLibraries/BPML_Global.TaskAddProgress` _array_element))
          (break)
          (elif (and (< _taskprogressextension _taskrequiredextension) _hasextension (`|EnumEquality` _boxtypeextension _type))
            (`KismetArrayLibrary.Array_Set` _text _array_index (`/Game/Code/ProjectLibraries/BPML_Global.TaskAddProgress` _array_element 1 "NewEnumerator1"))
            (break)))))
    (:`then_1`
      (`/Game/Code/wristGadget/RenderTargets/BP_text.Update Variables` (`self.TextManager`)))))

(fn `UserConstructionScript`)